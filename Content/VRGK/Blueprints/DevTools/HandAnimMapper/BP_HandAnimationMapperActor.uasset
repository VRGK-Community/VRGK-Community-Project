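; BP_HandAnimationMapperActor is a dev-tool actor that previews the stretched, opened and closed hand animations from a data asset on left and right hand meshes.
; Its construction script calls UpdateAnimationsFromDA in override mode to apply each pose animation to its mesh pair, then enables in-editor animation updates on all skeletal meshes.
; The same update event can use SetAnimation instead of overriding animation data.
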(event `CustomConstruction`
  (`self.UpdateAnimationsFromDA` (`self.Data Asset`) true)
  (`SkeletalMeshComponent.SetUpdateAnimationInEditor` (`self.K2_GetComponentsByClass` "/Script/Engine.SkeletalMeshComponent") true))

(event `UpdateAnimationsFromDA`
  (params (Target :type "/Game/VRGK/Blueprints/Data/BP_HandAnimationDataAsset Object Reference") (UseOverride :type Boolean))
  (bind _hand_stretched_animation (`/Game/VRGK/Blueprints/Data/BP_HandAnimationDataAsset.Hand Stretched Animation` Target))
  (bind _hand_opened_animation (`/Game/VRGK/Blueprints/Data/BP_HandAnimationDataAsset.Hand Opened Animation` Target))
  (bind _hand_closed_animation (`/Game/VRGK/Blueprints/Data/BP_HandAnimationDataAsset.Hand Closed Animation` Target))
  (`/Engine/EditorBlueprintResources/StandardMacros.IsValid` Target
    (:`Is Valid`
      (`|ExecutionSequence`
        (:`then_0`
          (if UseOverride
            (`SkeletalMeshComponent.OverrideAnimationData` (`self.RightStretched`) _hand_stretched_animation true true 0.0 1.0)
            (`SkeletalMeshComponent.OverrideAnimationData` (`self.LeftStretched`) _hand_stretched_animation true true 0.0 1.0)
            (else
              (`SkeletalMeshComponent.SetAnimation` (`self.LeftStretched`) _hand_stretched_animation)
              (`SkeletalMeshComponent.SetAnimation` (`self.RightStretched`) _hand_stretched_animation))))
        (:`then_1`
          (if UseOverride
            (`SkeletalMeshComponent.OverrideAnimationData` (`self.RightOpened`) _hand_opened_animation true true 0.0 1.0)
            (`SkeletalMeshComponent.OverrideAnimationData` (`self.LeftOpened`) _hand_opened_animation true true 0.0 1.0)
            (else
              (`SkeletalMeshComponent.SetAnimation` (`self.LeftOpened`) _hand_opened_animation)
              (`SkeletalMeshComponent.SetAnimation` (`self.RightOpened`) _hand_opened_animation))))
        (:`then_2`
          (if UseOverride
            (`SkeletalMeshComponent.OverrideAnimationData` (`self.RightClosed`) _hand_closed_animation true true 0.0 1.0)
            (`SkeletalMeshComponent.OverrideAnimationData` (`self.LeftClosed`) _hand_closed_animation true true 0.0 1.0)
            (else
              (`SkeletalMeshComponent.SetAnimation` (`self.LeftClosed`) _hand_closed_animation)
              (`SkeletalMeshComponent.SetAnimation` (`self.RightClosed`) _hand_closed_animation))))))))

(fn `UserConstructionScript`
  (`self.CustomConstruction`))