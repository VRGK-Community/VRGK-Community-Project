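; BP_DevT_HandPositioningHand is a developer-tool hand for VRGK hand positioning.
; On BeginPlay it orients the hand skeletal mesh by HandType, mirroring it with a negative Y scale for the left hand.
; Two events detach HandRoot and reattach it to DefaultSceneRoot while keeping its world transform, so the root and the hand can be moved independently.
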(event `self.ReceiveBeginPlay`
  (bind _handskeletalmesh (`self.HandSkeletalMesh`))
  (`|ExecutionSequence`
    (:`then_0`
      (switch `/Game/VRGK/Blueprints/Player/Hand/Enum_HandType` (`self.HandType`)
        (:`NewEnumerator0`
          (`SceneComponent.K2_SetRelativeRotation` (`self.HandSkeletalMesh`) (struct :`Roll` 90.0) false false))
        (:`NewEnumerator1`
          (`SceneComponent.SetRelativeScale3D` _handskeletalmesh (1.0 -1.0 1.0))
          (`SceneComponent.K2_SetRelativeRotation` _handskeletalmesh (struct :`Roll` -90.0) false false))))))

(event `DetachHandRoot`
  (`SceneComponent.K2_DetachFromComponent` (`self.HandRoot`) "KeepWorld" "KeepWorld" "KeepWorld" false))

(event `AttachHandRoot`
  (`SceneComponent.K2_AttachToComponent` (`self.HandRoot`) (`self.DefaultSceneRoot`) "None" "KeepWorld" "KeepWorld" "KeepWorld" false))

(fn `UserConstructionScript`)