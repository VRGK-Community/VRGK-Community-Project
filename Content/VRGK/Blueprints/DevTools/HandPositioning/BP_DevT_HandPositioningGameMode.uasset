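; Game mode for the VRGK hand positioning dev tool that owns the tool's save game object.
; On BeginPlay it loads the hand positioning save from a named slot, or creates a new one if none loads.
; On EndPlay it writes that object back to the same slot, so its data persists between sessions.
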(event `self.ReceiveBeginPlay`
  (bind _returnvalue (`GameplayStatics.LoadGameFromSlot` (`/Game/VRGK/Blueprints/DevTools/BPFL_DevTools.[DEVTOOLS] GetHandPosSlotName`)))
  (`/Engine/EditorBlueprintResources/StandardMacros.IsValid` _returnvalue
    (:`Is Valid`
      (bind _asbp_dev_t_save_game_hand_positioning (cast `/Game/VRGK/Blueprints/DevTools/HandPositioning/BP_DevT_SaveGame_HandPositioning` _returnvalue))
      (set `self.SaveGame` _asbp_dev_t_save_game_hand_positioning))
    (:`Is Not Valid`
      (bind _returnvalue_2 (`GameplayStatics.CreateSaveGameObject` "/Game/VRGK/Blueprints/DevTools/HandPositioning/BP_DevT_SaveGame_HandPositioning.BP_DevT_SaveGame_HandPositioning_C"))
      (set `self.SaveGame` _returnvalue_2))))

(event `self.ReceiveEndPlay`
  (params (EndPlayReason :type "EEndPlayReason Enum" :default "Destroyed"))
  (`GameplayStatics.SaveGameToSlot` (`self.SaveGame`) (`/Game/VRGK/Blueprints/DevTools/BPFL_DevTools.[DEVTOOLS] GetHandPosSlotName`)))

(fn `UserConstructionScript`)