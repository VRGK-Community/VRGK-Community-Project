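; VR dev-tool pawn for adjusting how the hands sit relative to the motion controllers.
; On BeginPlay it spawns a hand on each controller and restores the right hand root's offset from the game mode's SaveGame.
; Holding right grab detaches that hand root; releasing reattaches it at a new offset.
; MirrorFromHand copies the offset, axis-mirrored, to the other hand and stores the right-hand transform in the SaveGame object.
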(event `self.ReceiveBeginPlay`
  (bind (_handroottransform_location _handroottransform_rotation) (`KismetMathLibrary.BreakTransform` (`/Game/VRGK/Blueprints/DevTools/HandPositioning/BP_DevT_SaveGame_HandPositioning.HandRootTransform` (`/Game/VRGK/Blueprints/DevTools/HandPositioning/BP_DevT_HandPositioningGameMode.SaveGame` (cast `/Game/VRGK/Blueprints/DevTools/HandPositioning/BP_DevT_HandPositioningGameMode` (`GameplayStatics.GetGameMode`) :!pure true)))))
  (`parent.ReceiveBeginPlay`)
  (`|ExecutionSequence`
    (:`then_0`
      ;[1 1 1] Setup Hands
      (`|ExecutionSequence`
        (:`then_0`
          (bind _returnvalue (`|SpawnActorFromClass` "/Game/VRGK/Blueprints/DevTools/HandPositioning/BP_DevT_HandPositioningHand.BP_DevT_HandPositioningHand_C" (`KismetMathLibrary.MakeTransform` (0.0 0.0 0.0)) "Undefined" "OverrideRootScale" null "NewEnumerator0" null))
          (bind _output_get (set `self.RightHand` _returnvalue))
          (`self.K2_AttachToComponent` _output_get (`self.MotionControllerRight`) "None" "SnapToTarget" "SnapToTarget" "KeepWorld" false))
        (:`then_1`
          (bind _returnvalue_2 (`|SpawnActorFromClass` "/Game/VRGK/Blueprints/DevTools/HandPositioning/BP_DevT_HandPositioningHand.BP_DevT_HandPositioningHand_C" (`KismetMathLibrary.MakeTransform` (0.0 0.0 0.0)) "Undefined" "OverrideRootScale" null "NewEnumerator1" null))
          (bind _output_get_2 (set `self.LeftHand` _returnvalue_2))
          (`self.K2_AttachToComponent` _output_get_2 (`self.MotionControllerLeft`) "None" "SnapToTarget" "SnapToTarget" "KeepWorld" false))))
    (:`then_1`
      (`SceneComponent.K2_SetRelativeLocationAndRotation` (`/Game/VRGK/Blueprints/DevTools/HandPositioning/BP_DevT_HandPositioningHand.HandRoot` (`self.RightHand`)) _handroottransform_location _handroottransform_rotation false false)
      (`self.MirrorFromHand` "NewEnumerator0"))))

(event `InputAction|PlayerGrabRight`
  (params (Key :type "Key Structure"))
  (bind _righthand (`self.RightHand`))
  (:`Pressed`
    (`/Game/VRGK/Blueprints/DevTools/HandPositioning/BP_DevT_HandPositioningHand.DetachHandRoot` _righthand))
  (:`Released`
    (`/Game/VRGK/Blueprints/DevTools/HandPositioning/BP_DevT_HandPositioningHand.AttachHandRoot` _righthand)
    (`self.MirrorFromHand` "NewEnumerator0")))

(event `MirrorFromHand`
  (params (InitHand :type "/Game/VRGK/Blueprints/Player/Hand/Enum_HandType Enum" :default "NewEnumerator0"))
  (bind (_mirroredtransform_location _mirroredtransform_rotation) (`KismetMathLibrary.BreakTransform` (`/Game/VRGK/Blueprints/BPFL_GlobalFunctions.MirrorTransformByAxis` "NewEnumerator2" (`SceneComponent.GetRelativeTransform` (`/Game/VRGK/Blueprints/DevTools/HandPositioning/BP_DevT_HandPositioningHand.HandRoot` (select `/Game/VRGK/Blueprints/Player/Hand/Enum_HandType` InitHand :`NewEnumerator0` (`self.RightHand`) :`NewEnumerator1` (`self.LeftHand`)))))))
  (`SceneComponent.K2_SetRelativeLocationAndRotation` (`/Game/VRGK/Blueprints/DevTools/HandPositioning/BP_DevT_HandPositioningHand.HandRoot` (select `/Game/VRGK/Blueprints/Player/Hand/Enum_HandType` InitHand :`NewEnumerator0` (`self.LeftHand`) :`NewEnumerator1` (`self.RightHand`))) _mirroredtransform_location _mirroredtransform_rotation false false)
  (set `/Game/VRGK/Blueprints/DevTools/HandPositioning/BP_DevT_SaveGame_HandPositioning.HandRootTransform` (`SceneComponent.GetRelativeTransform` (`/Game/VRGK/Blueprints/DevTools/HandPositioning/BP_DevT_HandPositioningHand.HandRoot` (`self.RightHand`))) (`/Game/VRGK/Blueprints/DevTools/HandPositioning/BP_DevT_HandPositioningGameMode.SaveGame` (cast `/Game/VRGK/Blueprints/DevTools/HandPositioning/BP_DevT_HandPositioningGameMode` (`GameplayStatics.GetGameMode`) :!pure true))))

(fn `UserConstructionScript`
  (`parent.UserConstructionScript`))