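; BPO_Settings is the VR settings object, giving get/set access to vibration, standing and seated calibration, movement source, rotation options and world scale adjustment.
; Values live in PersistentSaveGame, and each setter writes there then fires a change dispatcher, without saving to disk itself.
; Height, seated mode and world scale setters share one calibration update that passes the settings object.
; Rotation speed is stored truncated to an integer but broadcast untruncated.
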(event `Init`)

(fn `GetRotationOptions`
  (returns (RotationType :type "/Game/VRGK/Blueprints/Player/PlayerCore/Enum_VRRotationOption Enum") (RotationSpeed :type "Float (double-precision)"))
  (bind _persistentsavegame (`self.PersistentSaveGame`))
  (return (`/Game/VRGK/Blueprints/Saves/BP_PersistentSaveGame.RotationType` _persistentsavegame) (`KismetMathLibrary.Conv_IntToDouble` (`/Game/VRGK/Blueprints/Saves/BP_PersistentSaveGame.RotationSpeed` _persistentsavegame))))

(fn `GetSeatedPlayerHeight`
  (returns (SittingPlayerHeight :type "Float (double-precision)"))
  (return (`/Game/VRGK/Blueprints/Saves/BP_PersistentSaveGame.SeatedPlayerHeight` (`self.PersistentSaveGame`))))

(fn `GetSeatedPlayModeEnabled`
  (returns (Enabled :type Boolean))
  (return (`/Game/VRGK/Blueprints/Saves/BP_PersistentSaveGame.SeatedPlayModeEnabled` (`self.PersistentSaveGame`))))

(fn `GetStandingPlayerHeight`
  (returns (StandingPlayerHeight :type "Float (double-precision)"))
  (return (`/Game/VRGK/Blueprints/Saves/BP_PersistentSaveGame.StandingPlayerHeight` (`self.PersistentSaveGame`))))

(fn `GetVibrationEnabled`
  (returns (VibrationEnabeld :type Boolean))
  (return (`/Game/VRGK/Blueprints/Saves/BP_PersistentSaveGame.VibrationEnabeld` (`self.PersistentSaveGame`))))

(fn `GetVRMovementSource`
  (returns (`Current Movement Source` :type "/Game/VRGK/Blueprints/Player/PlayerCore/Enum_VRMovementSource Enum"))
  (return (`/Game/VRGK/Blueprints/Saves/BP_PersistentSaveGame.VRMovementSource` (`self.PersistentSaveGame`))))

(fn `GetWorldScaleAdjustmentEnabled`
  (returns (Enabled :type Boolean))
  (return (`/Game/VRGK/Blueprints/Saves/BP_PersistentSaveGame.WorldScaleAdjustmentEnabled` (`self.PersistentSaveGame`))))

(fn `SetRotationOptions`
  (params (NewType :type "/Game/VRGK/Blueprints/Player/PlayerCore/Enum_VRRotationOption Enum" :default "NewEnumerator0") (NewSpeed :type "Float (double-precision)"))
  (bind _persistentsavegame (`self.PersistentSaveGame`))
  (bind _output_get (set `/Game/VRGK/Blueprints/Saves/BP_PersistentSaveGame.RotationType` NewType _persistentsavegame))
  (set `/Game/VRGK/Blueprints/Saves/BP_PersistentSaveGame.RotationSpeed` (`KismetMathLibrary.FTrunc` NewSpeed) _persistentsavegame)
  (`self.OnRotationOptionsChanged` _output_get NewSpeed))

(fn `SetSeatedPlayerHeight`
  (params (NewSittingHeight :type "Float (double-precision)"))
  (set `/Game/VRGK/Blueprints/Saves/BP_PersistentSaveGame.SeatedPlayerHeight` NewSittingHeight (`self.PersistentSaveGame`))
  (`self.OnPlayerCalibrationUpdate` self))

(fn `SetSeatedPlayModeEnabled`
  (params (Enabled :type Boolean))
  (set `/Game/VRGK/Blueprints/Saves/BP_PersistentSaveGame.SeatedPlayModeEnabled` Enabled (`self.PersistentSaveGame`))
  (`self.OnPlayerCalibrationUpdate` self))

(fn `SetStandingPlayerHeight`
  (params (NewHeight :type "Float (double-precision)"))
  (set `/Game/VRGK/Blueprints/Saves/BP_PersistentSaveGame.StandingPlayerHeight` NewHeight (`self.PersistentSaveGame`))
  (`self.OnPlayerCalibrationUpdate` self))

(fn `SetVibrationEnabled`
  (params (Enabled :type Boolean))
  (bind _output_get (set `/Game/VRGK/Blueprints/Saves/BP_PersistentSaveGame.VibrationEnabeld` Enabled (`self.PersistentSaveGame`)))
  (`self.OnVibrationEnabled` _output_get))

(fn `SetVRMovementSource`
  (params (NewMovementSource :type "/Game/VRGK/Blueprints/Player/PlayerCore/Enum_VRMovementSource Enum" :default "NewEnumerator0"))
  (bind _output_get (set `/Game/VRGK/Blueprints/Saves/BP_PersistentSaveGame.VRMovementSource` NewMovementSource (`self.PersistentSaveGame`)))
  (`self.OnVRMovementSourceChange` _output_get))

(fn `SetWorldScaleAdjustmentEnabled`
  (params (Enabled :type Boolean))
  (set `/Game/VRGK/Blueprints/Saves/BP_PersistentSaveGame.WorldScaleAdjustmentEnabled` Enabled (`self.PersistentSaveGame`))
  (`self.OnPlayerCalibrationUpdate` self))