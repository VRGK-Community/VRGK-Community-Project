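; VR player component that tracks gravity state: whether gravity is on, whether custom directions apply, and the current direction and multiplier.
; Setters update that state and fire dispatchers for enable and direction changes.
; Tick runs only while custom directions are active or set to always update, broadcasting direction scaled by multiplier and default strength.
; The direction getter falls back to world down when custom directions are off.
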(event `self.ReceiveBeginPlay`
  (`self.RefreshGravityStatus`))

(event `RefreshGravityStatus`
  (`self.SetCustomGravityDirectionsEnabled` (`self.CustomGravityEnabled`))
  (`self.SetPlayerGravityEnabled` (`self.PlayerGravityEnabled`)))

(event `self.ReceiveTick`
  (params (DeltaSeconds :type "Float (single-precision)"))
  (`self.OnGravityUpdate` (* (`self.GravityDirection`) (* (`self.GravityMultiplier`) (`self.DefaultGravityStrength`)))))

(event `SetCustomGravityDirectionsEnabled`
  (params (Enabled :type Boolean))
  (set `self.CustomGravityEnabled` Enabled)
  (if (or (`self.Is Gravity With Custom Directions Enabled`) (and (`self.CustomGravityEnabled`) (`self.AlwaysDoCustomDirectionUpdates`)))
    (`self.SetComponentTickEnabled` true)
    (`self.OnCustomGravityDirectionEnabled` true)
    (else
      (`self.SetComponentTickEnabled` false)
      (`self.OnCustomGravityDirectionEnabled` false))))

(event `SetPlayerGravityEnabled`
  (params (`Gravity Enabled` :type Boolean))
  (set `self.PlayerGravityEnabled` `Gravity Enabled`)
  (`self.SetCustomGravityDirectionsEnabled` (`self.CustomGravityEnabled`))
  (`self.OnGravityEnabled` (`self.PlayerGravityEnabled`) (`self.CustomGravityEnabled`)))

(event `SetNewGravityDirection`
  (params (`New Gravity Direction` :type "Vector Structure"))
  (bind _output_get (set `self.GravityDirection` `New Gravity Direction`))
  (`self.OnGravityDirectionChanged` _output_get))

(event `SetNewGravityMultiplier`
  (params (`New Multiplier` :type "Float (double-precision)"))
  (set `self.GravityMultiplier` `New Multiplier`))

(fn `GetGravityDirection`
  (returns (Direction :type "Vector Structure"))
  (return (`KismetMathLibrary.SelectVector` (`self.GravityDirection`) (0.0 0.0 -1.0) (or (`self.CustomGravityEnabled`) (and (`self.CustomGravityEnabled`) (`self.AlwaysDoCustomDirectionUpdates`))))))

(fn `Is Custom Gravity Directions Enabled`
  (returns (True :type Boolean))
  (return (`self.CustomGravityEnabled`)))

(fn `Is Gravity With Custom Directions Enabled`
  (returns (True :type Boolean))
  (return (and (`self.CustomGravityEnabled`) (`self.PlayerGravityEnabled`))))

(fn `IsGravityEnabled`
  (returns (True :type Boolean))
  (return (`self.PlayerGravityEnabled`)))