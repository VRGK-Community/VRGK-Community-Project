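; Physics body rig for the VR physics pawn, built from constrained fender sphere, locomotion sphere, body capsule and head sphere, with both physics hands attached.
; Each tick it drives head and capsule from tracked height, updates hand constraints and traces for ground.
; Ground contact scales the locomotion sphere up or down.
; Slope, speed, input and collisions select its friction material, allowing quick stops yet sliding on slopes.
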(event `self.ReceiveBeginPlay`
  ;[0.232 1 0.619 1 32] BeginPlay
  (`self.SetPhysicsRigGravityEnabled` (`self.IsGravityEnabled`))
  (`self.SetCollisionPartsVisibility` false)
  (`/Engine/EditorBlueprintResources/StandardMacros.IsValid` (`self.PhysicsPawnParent`)
    (:`Is Valid`
      (`self.SetupPhysicsBody`)
      (`self.SetLocomotionSphereScale` 0.0)
      (`self.DoLocomotionSphereScaleUp`))
    (:`Is Not Valid`
      (`self.SetActorTickEnabled` false))))

(event `SetupLocomotionSphere`
  ;[1 1 1] Manual Setup Locomotion Sphere
  (`self.ManualSetupConstraint` (`self.LocomotionSphereConstraint`) (`self.LocomotionSphere`) (`self.FenderSphere`) (struct) (`KismetMathLibrary.MakeTransform` (`SceneComponent.RelativeLocation` (`self.LocomotionSphereConstraint`)))))

(event `self.ReceiveTick`
  (params (DeltaSeconds :type "Float (single-precision)"))
  ;[1 0.5399 0.3313 1 32] Event Tick
  (`|ExecutionSequence`
    (:`then_0`
      (`self.UpdatePhysicsHeadConstraints`)
      (`/Game/VRGK/Blueprints/Player/GamePawns/BP_VRHand_PhysicsPawn.UpdateHandConstraintFrames` (`self.LeftPhysicsHand`))
      (`/Game/VRGK/Blueprints/Player/GamePawns/BP_VRHand_PhysicsPawn.UpdateHandConstraintFrames` (`self.RightPhysicsHand`))
      (`self.UpdateBodyCapsule`))
    (:`then_1`
      (`self.CalculateHeadTargetOffset`)
      (`self.CheckIfPlayerIsTouchingGround`)
      (`self.UpdateLocomotionFriction` DeltaSeconds))
    (:`then_2`
      (`self.OnFinalizePhysicsRigEventTick` DeltaSeconds))))

(event `SetupPhysicsBody`
  (bind _headsphereconstraint (`self.HeadSphereConstraint`))
  ;[1 1 1] Setup Physics Body
  (`|ExecutionSequence`
    (:`then_0`
      (`PhysicsConstraintComponent.BreakConstraint` (`self.BodyCapsuleConstraint`))
      (`PhysicsConstraintComponent.BreakConstraint` (`self.LocomotionSphereConstraint`))
      (`PhysicsConstraintComponent.BreakConstraint` (`self.HeadSphereConstraint`))
      (`self.SetupHeadSphere`))
    (:`then_1`
      (`self.SetupHands`)
      (`PhysicsConstraintComponent.SetConstraintReferenceFrame` _headsphereconstraint "Frame1" (`KismetMathLibrary.MakeTransform` (0.0 0.0 0.0)))
      (`PhysicsConstraintComponent.SetConstraintReferenceFrame` _headsphereconstraint "Frame2" (`KismetMathLibrary.MakeTransform` (0.0 0.0 0.0))))
    (:`then_2`
      (`self.SetupBodyCapsule`)
      (`self.SetupLocomotionSphere`))
    (:`then_3`
      (`self.SetupTickPrerequisiteHands`))))

(event `SetupBodyCapsule`
  (bind _bodycapsuleconstraint (`self.BodyCapsuleConstraint`))
  ;[1 1 1] Manual Setup Locomotion Sphere
  (`self.ManualSetupConstraint` _bodycapsuleconstraint (`self.BodyCapsule`) (`self.FenderSphere`) (`KismetMathLibrary.MakeTransform` (0.0 0.0 -40.0)) (`KismetMathLibrary.MakeTransform` (`SceneComponent.RelativeLocation` _bodycapsuleconstraint))))

(event `CalculateHeadTargetOffset`
  (bind (_returnvalue_location _returnvalue_rotation _returnvalue_scale) (`KismetMathLibrary.BreakTransform` (`SceneComponent.K2_GetComponentToWorld` (`self.HeadSphereConstraint`))))
  (bind (_returnvalue_x _returnvalue_y _returnvalue_z) (`KismetMathLibrary.BreakVector` (`KismetMathLibrary.InverseTransformLocation` (`KismetMathLibrary.MakeTransform` _returnvalue_location _returnvalue_rotation _returnvalue_scale) (`SceneComponent.K2_GetComponentLocation` (`self.HeadSphere`)))))
  (bind _returnvalue (- (`self.Calculate Adjusted Head Height` (`self.TargetRigHeight`)) _returnvalue_z))
  ;[0.4364 0.6266 1] Calculate current Offset between Target Head Height and actual Head Height
  (set `self.CurrentHeadTargetOffset` (`KismetMathLibrary.MapRangeClamped` (`KismetMathLibrary.Abs` _returnvalue) 5.0 10.0 0.0 _returnvalue)))

(event `self.BPC_GravityAreaFinder.OnGravityUpdate`
  (params (`Current Gravity` :type "Vector Structure") (Strength :type "Float (single-precision)"))
  (bind _bp_vrgravitytracker (`/Game/VRGK/Blueprints/Player/GamePawns/BP_VRPhysicsPawn.BP_VRGravityTracker` (`self.PhysicsPawnParent`)))
  ;[1 0.4126 0.9053] Update Gravity Information from Area Finder
  (`/Game/VRGK/Blueprints/Player/BPC_VRGravityTracker.SetNewGravityDirection` _bp_vrgravitytracker `Current Gravity`)
  (`/Game/VRGK/Blueprints/Player/BPC_VRGravityTracker.SetNewGravityMultiplier` _bp_vrgravitytracker Strength))

(event `SetupHeadSphere`
  ;[1 1 1] Manual Setup Locomotion Sphere
  (`self.ManualSetupConstraint` (`self.HeadSphereConstraint`) (`self.HeadSphere`) (`self.FenderSphere`)))

(event `self.HeadSphere.OnComponentHit`
  (params (HitComponent :type "PrimitiveComponent Object Reference") (OtherActor :type "Actor Object Reference") (OtherComp :type "PrimitiveComponent Object Reference") (NormalImpulse :type "Vector Structure") (Hit :type "HitResult Structure (by ref)"))
  ;[1 0.5804 0.3462] Check if Head is Colliding
  (`/Engine/EditorBlueprintResources/StandardMacros.DoOnce` false :!label _label
    (:`Completed`
      (`|ExecutionSequence`
        (:`then_0`
          (set `self.HeadSphereIsColliding` true)
          (`KismetSystemLibrary.RetriggerableDelay` 0.05)
          (set `self.HeadSphereIsColliding` false))
        (:`then_1`
          (`KismetSystemLibrary.Delay` 0.0)
          (goto _label :!via `Reset`))))))

(event `UpdateLocomotionFriction`
  (params (`Delta Seconds` :type "Float (double-precision)"))
  ;[0.1041 0.7808 1] Update Locomotion Sphere Friction with different Physical Materials. Helps to stop fast during Controller Movement while moving on ground, but keeps sliding of Slopes possible.
  (bind (_recommended_phys_mat _change_speed) (`self.GetRecommendedLocomotionFrictionMaterial`))
  (if (!= (`self.CurrentLocomotionPhysicalMaterial`) _recommended_phys_mat)
    (if (> (- (`self.GetGameTimeSinceCreation`) (`self.LocomotionFrictionChangeTime`)) _change_speed)
      (bind _output_get (set `self.CurrentLocomotionPhysicalMaterial` _recommended_phys_mat))
      (`PrimitiveComponent.SetPhysMaterialOverride` (`self.LocomotionSphere`) _output_get) ; Set Weak Material
      (set `self.LocomotionFrictionChangeTime` (`self.GetGameTimeSinceCreation`)))
    (else
      (set `self.LocomotionFrictionChangeTime` (`self.GetGameTimeSinceCreation`)))))

(event `self.LocomotionSphere.OnComponentHit`
  (params (HitComponent :type "PrimitiveComponent Object Reference") (OtherActor :type "Actor Object Reference") (OtherComp :type "PrimitiveComponent Object Reference") (NormalImpulse :type "Vector Structure") (Hit :type "HitResult Structure (by ref)"))
  ;[1 0.5857 0.2406] Check if Locomotion Sphere is Colliding
  (`/Engine/EditorBlueprintResources/StandardMacros.DoOnce` false :!label _label_2
    (:`Completed`
      (`|ExecutionSequence`
        (:`then_0`
          (`|ExecutionSequence`
            (:`then_0`
              (if (not (`self.LocomotionSphereIsColliding`))
                (set `self.LocomotionSphereIsColliding` true)))
            (:`then_1`
              (`KismetSystemLibrary.RetriggerableDelay` 0.2)
              (if (`self.LocomotionSphereIsColliding`)
                (set `self.LocomotionSphereIsColliding` false)))))
        (:`then_1`
          (`KismetSystemLibrary.Delay` 0.0)
          (goto _label_2 :!via `Reset`))))))

(event `self.FenderSphere.OnComponentHit`
  (params (HitComponent :type "PrimitiveComponent Object Reference") (OtherActor :type "Actor Object Reference") (OtherComp :type "PrimitiveComponent Object Reference") (NormalImpulse :type "Vector Structure") (Hit :type "HitResult Structure (by ref)"))
  ;[1 0.3399 0.214] Check if Fender Sphere is Colliding
  (`/Engine/EditorBlueprintResources/StandardMacros.DoOnce` false :!label _label_3
    (:`Completed`
      (`|ExecutionSequence`
        (:`then_0`
          (`|ExecutionSequence`
            (:`then_0`
              (if (not (`self.FenderSphereIsColliding`))
                (set `self.FenderSphereIsColliding` true)))
            (:`then_1`
              (`KismetSystemLibrary.RetriggerableDelay` 0.2)
              (if (`self.FenderSphereIsColliding`)
                (set `self.FenderSphereIsColliding` false)))))
        (:`then_1`
          (`KismetSystemLibrary.Delay` 0.0)
          (goto _label_3 :!via `Reset`))))))

(event `SetCollisionPartsVisibility`
  (params (Visible :type Boolean))
  ;[1 1 1] Set Visibility of Collision parts.
  (`SceneComponent.SetHiddenInGame` (`self.LocomotionSphere`) (not Visible) false)
  (`SceneComponent.SetHiddenInGame` (`self.FenderSphere`) (not Visible) false)
  (`SceneComponent.SetHiddenInGame` (`self.BodyCapsule`) (not Visible) false)
  (`SceneComponent.SetHiddenInGame` (`self.HeadSphere`) (not Visible) false))

(event `UpdatePhysicsHeadConstraints`
  (bind _headsphereconstraint (`self.HeadSphereConstraint`))
  (bind (_returnvalue_location _returnvalue_rotation _returnvalue_scale) (`KismetMathLibrary.BreakTransform` (`SceneComponent.K2_GetComponentToWorld` _headsphereconstraint)))
  (bind (_returnvalue_x _returnvalue_y) (`KismetMathLibrary.BreakVector` (* (* (`KismetMathLibrary.InverseTransformLocation` (`KismetMathLibrary.MakeTransform` _returnvalue_location _returnvalue_rotation _returnvalue_scale) (`SceneComponent.K2_GetComponentLocation` (`/Game/VRGK/Blueprints/Player/GamePawns/BP_VRPhysicsPawn.HeadRoot` (`self.PhysicsPawnParent`)))) (`/Game/VRGK/Blueprints/Player/PlayerCore/BP_VRGamePawn.GetVRPawnWorldScale` (`self.PhysicsPawnParent`))) -1.0)))
  ;[1 0.6016 0.3585] Update Head Constraints
  (`PhysicsConstraintComponent.SetLinearPositionTarget` (`self.HeadSphereConstraint`) (`KismetMathLibrary.MakeVector` 0.0 0.0 (* (`self.Calculate Adjusted Head Height Clamped` (`self.TargetRigHeight`)) (`/Game/VRGK/Blueprints/Player/PlayerCore/BP_VRGamePawn.GetVRPawnWorldScale` (`self.PhysicsPawnParent`)))))
  (`PhysicsConstraintComponent.SetConstraintReferenceFrame` _headsphereconstraint "Frame1" (`KismetMathLibrary.MakeTransform` (`KismetMathLibrary.MakeVector` _returnvalue_x _returnvalue_y))))

(event `UpdateRigBodyConstraintFrames`
  (bind _bodycapsuleconstraint (`self.BodyCapsuleConstraint`))
  (bind _locomotionsphereconstraint (`self.LocomotionSphereConstraint`))
  ;[1 0.2812 0.2911] Update all Constraint Frames with current Scaling and other Adjustments
  (`self.PhysicsPawnParent`
    (:`then`
      (`|ExecutionSequence`
        (:`then_0`
          ;;[1 1 1] Locomotion Sphere Constraint Frame
          (`PhysicsConstraintComponent.SetConstraintReferenceFrame` _locomotionsphereconstraint "Frame2" (`KismetMathLibrary.MakeTransform` (* (`SceneComponent.RelativeLocation` _locomotionsphereconstraint) (`/Game/VRGK/Blueprints/Player/PlayerCore/BP_VRGamePawn.GetVRPawnWorldScale` (`self.PhysicsPawnParent`)))))
          (`PhysicsConstraintComponent.SetConstraintReferenceFrame` (`self.LocomotionSphereConstraint`) "Frame1" (`KismetMathLibrary.MakeTransform` (0.0 0.0 0.0))))
        (:`then_1`
          ;;[1 1 1] Body Capsule Constraint Frame
          (`PhysicsConstraintComponent.SetConstraintReferenceFrame` _bodycapsuleconstraint "Frame2" (`KismetMathLibrary.MakeTransform` (* (`SceneComponent.RelativeLocation` _bodycapsuleconstraint) (`/Game/VRGK/Blueprints/Player/PlayerCore/BP_VRGamePawn.GetVRPawnWorldScale` (`self.PhysicsPawnParent`)))))
          (`PhysicsConstraintComponent.SetConstraintReferenceFrame` (`self.LocomotionSphereConstraint`) "Frame1" (`KismetMathLibrary.MakeTransform` (0.0 0.0 0.0))))
        (:`then_2`
          (`PhysicsConstraintComponent.SetConstraintReferenceFrame` (`self.HeadSphereConstraint`) "Frame2" (`KismetMathLibrary.MakeTransform` (0.0 0.0 0.0))))))
    (:`else`)))

(event `SetConstraintJumpModeEnabled`
  (params (Enabled :type Boolean))
  ;[0.5616 1 0.5171] Enables Jumping Mode for Head Constraint. Without this, the Pawn would not actually jump high.
  (`PhysicsConstraintComponent.SetLinearDriveParams` (`self.HeadSphereConstraint`) (`KismetMathLibrary.SelectFloat` 10000.0 5000.0 Enabled) (`KismetMathLibrary.SelectFloat` 0.0 100.0 Enabled) 0.0))

(event `AttachHandsToPhysicsRig`
  (params (`VR Hand` :type "/Game/VRGK/Blueprints/Player/GamePawns/BP_VRHand_PhysicsPawn Object Reference"))
  ;[0.3993 0.4175 1] Attach Hands to the Physics Rig
  (`/Game/VRGK/Blueprints/Player/Hand/BP_VRHand.ReconstraintHandConstraints` `VR Hand`)
  (`/Game/VRGK/Blueprints/Player/Hand/BP_VRHand.ResetPDConstraintAttachments` `VR Hand`))

(event `SetupHands`
  ;[0.4485 0.6755 1] Setup Physics Rig VRHands
  (set `self.LeftPhysicsHand` (cast `/Game/VRGK/Blueprints/Player/GamePawns/BP_VRHand_PhysicsPawn` (`/Game/VRGK/Blueprints/Player/PlayerCore/BP_VRGamePawn.LeftHand` (`self.PhysicsPawnParent`)) :!pure true))
  (set `self.RightPhysicsHand` (cast `/Game/VRGK/Blueprints/Player/GamePawns/BP_VRHand_PhysicsPawn` (`/Game/VRGK/Blueprints/Player/PlayerCore/BP_VRGamePawn.RightHand` (`self.PhysicsPawnParent`)) :!pure true))
  (bind _output_get (set `/Game/VRGK/Blueprints/Player/GamePawns/BP_VRHand_PhysicsPawn.PhysicsRig` self (`self.RightPhysicsHand`)))
  (set `/Game/VRGK/Blueprints/Player/GamePawns/BP_VRHand_PhysicsPawn.PhysicsRig` _output_get (`self.LeftPhysicsHand`))
  (`self.AttachHandsToPhysicsRig` (`self.RightPhysicsHand`))
  (`self.AttachHandsToPhysicsRig` (`self.LeftPhysicsHand`)))

(event `SetupTickPrerequisiteHands`
  ;[0.1999 0.9901 1] Tick Prerequisites for Hands
  (`self.AddTickPrerequisiteActor` self (`self.RightPhysicsHand`))
  (`self.AddTickPrerequisiteActor` self (`self.LeftPhysicsHand`)))

(event `UpdateBodyCapsule`
  ;[1 0.3777 0.7951] Update Body Capsule and Size
  (set `self.LocalNeckLocation` (* (`KismetMathLibrary.InverseTransformLocation` (`SceneComponent.K2_GetComponentToWorld` (`self.FenderSphere`)) (`SceneComponent.K2_GetComponentLocation` (`self.NeckRoot`))) (0.0 0.0 1.0)))
  (`CapsuleComponent.SetCapsuleHalfHeight` (`self.BodyCapsule`) (`KismetMathLibrary.FInterpTo_Constant` (`CapsuleComponent.CapsuleHalfHeight` (`self.BodyCapsule`)) (+ (/ (`KismetMathLibrary.FMax` (`KismetMathLibrary.VSize` (`self.LocalNeckLocation`)) 20.0) 2.0) (`CapsuleComponent.CapsuleRadius` (`self.BodyCapsule`))) (`GameplayStatics.GetWorldDeltaSeconds`) 200.0) true)
  (bind _output_get (set `self.LastBodyConstraintPosition` (`KismetMathLibrary.VInterpTo_Constant` (`self.LastBodyConstraintPosition`) (`KismetMathLibrary.NegateVector` (/ (`self.LocalNeckLocation`) 2.0)) (`GameplayStatics.GetWorldDeltaSeconds`) 200.0)))
  (`PhysicsConstraintComponent.SetConstraintReferencePosition` (`self.BodyCapsuleConstraint`) "Frame1" (* _output_get (`/Game/VRGK/Blueprints/Player/PlayerCore/BP_VRGamePawn.GetVRPawnWorldScale` (`self.PhysicsPawnParent`)))))

(event `SetLocomotionSphereScale`
  (params (`Scale Alpha` :type "Float (double-precision)"))
  (bind _returnvalue (`KismetMathLibrary.FClamp` `Scale Alpha`))
  ;[0.1402 0.671 1] Locomotion Sphere Scaling
  (`SphereComponent.SetSphereRadius` (`self.FenderSphere`) (`KismetMathLibrary.Lerp` 10.0 20.0 _returnvalue) true)
  (`SphereComponent.SetSphereRadius` (`self.LocomotionSphere`) (`KismetMathLibrary.Lerp` 10.0 (`self.MaxLocomotionSphereRadius`) _returnvalue) true))

(event `DoLocomotionSphereScaleUp`
  ;[0.1402 0.671 1] Locomotion Sphere Scaling
  (bind (_direction _scale_alpha) (`Timeline|LocomotionSphereScalingTimeline` :!label _label)
    (:`Update`
      _)
    (:`Finished`
      _))
  (`self.SetLocomotionSphereScale` _scale_alpha))

(event `DoLocomotionSphereScaleDown`
  ;[0.1402 0.671 1] Locomotion Sphere Scaling
  (goto _label :!via `Reverse`))

(event `CheckIfPlayerIsTouchingGround`
  (bind _returnvalue (`SceneComponent.K2_GetComponentLocation` (`self.LocomotionSphereConstraint`)))
  (bind _returnvalue_2 (`SceneComponent.K2_GetComponentLocation` (`self.LocomotionSphereConstraint`)))
  (bind _returnvalue_3 (`SphereComponent.GetScaledSphereRadius` (`self.LocomotionSphere`)))
  (bind _current_scale (`/Game/VRGK/Blueprints/Player/PlayerCore/BP_VRGamePawn.GetVRPawnWorldScale` (`self.PhysicsPawnParent`)))
  (bind _returnvalue_4 (* _returnvalue_3 0.8))
  ;[1 0.4564 0.04679] Check for Ground on the Physics Pawn.
  (bind (_outhit _returnvalue_5) (`KismetSystemLibrary.SphereTraceSingleByProfile` _returnvalue_2 (- _returnvalue_2 (* (* (`SceneComponent.GetUpVector` (`self.FenderSphere`)) (`self.MaxLocomotionSphereRadius`)) _current_scale)) (* (`self.GroundCheckRadius`) _current_scale) "VRPhysicsPawn"))
  (`|ExecutionSequence`
    (:`then_0`
      (if _returnvalue_5
        (set `self.LastLocomotionGroundHitResult` _outhit)
        (`self.DoTouchingGround`)
        (else
          (bind (_outhit_2 _returnvalue_6) (`KismetSystemLibrary.SphereTraceSingleByProfile` _returnvalue (- _returnvalue (* (`SceneComponent.GetUpVector` (`self.FenderSphere`)) (+ (* (`/Game/VRGK/Blueprints/Player/PlayerCore/BP_VRGamePawn.GetVRPawnWorldScale` (`self.PhysicsPawnParent`)) 5.0) (- _returnvalue_3 _returnvalue_4)))) _returnvalue_4 "VRPhysicsPawn")) ; Do a second bigger Trace that is only used to check if something is near the Locomotion Sphere.\n\nUse case: Reducing LocoSphere Scaling moments to the minimum.
          (if _returnvalue_6
            (set `self.LastLocomotionGroundHitResult` _outhit_2)
            (`self.DoTouchingGround`)))))
    (:`then_1`
      (`/Game/VRGK/Blueprints/Player/GamePawns/BP_VRPhysicsPawn.UpdateGroundObjectInfo` (`self.PhysicsPawnParent`) _outhit _returnvalue_5))))

(event `DoTouchingGround`
  ;[1 0.4564 0.04679] Check for Ground on the Physics Pawn.
  (`|ExecutionSequence`
    (:`then_0`
      (if (not (`self.IsTouchingGround`))
        (set `self.IsTouchingGround` true)
        (`self.OnTouchingGround` true)
        (`self.DoLocomotionSphereScaleUp`)))
    (:`then_1`
      (`KismetSystemLibrary.RetriggerableDelay` 0.1)
      (if (`self.IsTouchingGround`)
        (set `self.IsTouchingGround` false)
        (`self.OnTouchingGround` false)
        (`self.DoLocomotionSphereScaleDown`)))))

(fn `AddForceToPhysicsRig`
  (params (Force :type "Vector Structure") (bAccelChange :type Boolean))
  (`PrimitiveComponent.AddForce` (`self.FenderSphere`) Force "None" bAccelChange)
  (`PrimitiveComponent.AddForce` (`self.BodyCapsule`) Force "None" bAccelChange)
  (`PrimitiveComponent.AddForce` (`self.HeadSphere`) Force "None" bAccelChange)
  (`PrimitiveComponent.AddForce` (`self.LocomotionSphere`) Force "None" bAccelChange))

(fn `AddLocomotionTorque`
  (params (Torque :type "Vector Structure") (bAccelChange :type Boolean))
  (if (not (`KismetMathLibrary.Vector_IsNearlyZero` Torque 0.001))
    (`PrimitiveComponent.AddTorqueInDegrees` (`self.LocomotionSphere`) Torque "None" bAccelChange)))

(fn `AddRigWorldOffset`
  (params (DeltaLocation :type "Vector Structure") (bSweep :type Boolean) (bTeleport :type Boolean))
  (locals (TempLocoSphereRadius :type "Float (double-precision)" :default 0.0))
  (`|ExecutionSequence`
    (:`then_0`
      ;[1 1 1] Scale down the Locomotion Sphere to reduce issues by manually moving the Rig.
      (if (`self.ScaleDownLocomotionSphereDuringAddOffsets`)
        (bind _output_get (set `local.TempLocoSphereRadius` (`SphereComponent.SphereRadius` (`self.LocomotionSphere`))))
        (`SphereComponent.SetSphereRadius` (`self.LocomotionSphere`) (* _output_get 0.8) false)))
    (:`then_1`
      (`SceneComponent.K2_AddWorldOffset` (`self.FenderSphere`) (`local.DeltaLocation`) (`local.bSweep`) (`local.bTeleport`))
      (`SceneComponent.K2_AddWorldOffset` (`self.BodyCapsule`) (`local.DeltaLocation`) (`local.bSweep`) (`local.bTeleport`))
      (`SceneComponent.K2_AddWorldOffset` (`self.HeadSphere`) (`local.DeltaLocation`) (`local.bSweep`) (`local.bTeleport`))
      (`SceneComponent.K2_AddWorldOffset` (`self.LocomotionSphere`) (`local.DeltaLocation`) (`local.bSweep`) (`local.bTeleport`)))
    (:`then_2`
      ;[1 1 1] Scale the Loco Sphere back, after the Offset has been added.
      (if (`self.ScaleDownLocomotionSphereDuringAddOffsets`)
        (`SphereComponent.SetSphereRadius` (`self.LocomotionSphere`) (`local.TempLocoSphereRadius`) false)))))

(fn `Calculate Adjusted Head Height`
  (params (Height :type "Float (double-precision)"))
  (returns (Calculated :type "Float (double-precision)"))
  (bind (_relativelocation_x _relativelocation_y _relativelocation_z) (`KismetMathLibrary.BreakVector` (`SceneComponent.RelativeLocation` (`self.LocomotionSphereConstraint`))))
  (return (`KismetMathLibrary.FMax` (+ (- Height (`self.MaxLocomotionSphereRadius`)) _relativelocation_z))))

(fn `Calculate Adjusted Head Height Clamped`
  (params (Height :type "Float (double-precision)"))
  (returns (Calculated :type "Float (double-precision)"))
  (return (`KismetMathLibrary.FClamp` (`self.Calculate Adjusted Head Height` Height) 0.0 (`KismetMathLibrary.FMin` (+ (`self.MaximumRigHeight`) 10.0) (`self.FixedMaximumBodyHeight`) (`self.FixedMaximumBodyHeight`)))))

(fn `Get Hand Socket Relative Frame`
  (params (`Target Hand` :type "/Game/VRGK/Blueprints/Player/Hand/BP_VRHand Object Reference"))
  (returns (FrameT :type "Transform Structure"))
  (bind _returnvalue (`SceneComponent.K2_GetComponentToWorld` (`/Game/VRGK/Blueprints/Player/Hand/BP_VRHand.HandSocket` `Target Hand`)))
  (bind (_returnvalue_location _returnvalue_rotation) (`KismetMathLibrary.BreakTransform` (`SceneComponent.K2_GetComponentToWorld` (`/Game/VRGK/Blueprints/Player/Hand/BP_VRHand.HandRoot` `Target Hand`))))
  (return (`KismetMathLibrary.MakeTransform` (`KismetMathLibrary.InverseTransformLocation` _returnvalue _returnvalue_location) (`KismetMathLibrary.InverseTransformRotation` _returnvalue _returnvalue_rotation))))

(fn `GetHandCenter`
  (returns (Sphere :type "SphereComponent Object Reference"))
  (return (`self.FenderSphere`)))

(fn `GetRecommendedLocomotionFrictionMaterial`
  (returns (`Recommended Phys Mat` :type "PhysicalMaterial Object Reference") (`Change Speed` :type "Float (double-precision)"))
  (locals (GroundDot :type "Float (double-precision)" :default 0.0) (RecommendedStrong :type "PhysicalMaterial Object Reference" :default "PhysicalMaterial'/Game/VRGK/PhysicalMaterials/Player/PM_PhysicsPawn_LocomotionSphere_Normal.PM_PhysicsPawn_LocomotionSphere_Normal'") (RecommendedWeak :type "PhysicalMaterial Object Reference" :default "PhysicalMaterial'/Game/VRGK/PhysicalMaterials/Player/PM_PhysicsPawn_LocomotionSphere_Normal.PM_PhysicsPawn_LocomotionSphere_Normal'") (TargetWeakChangeSpeed :type "Float (double-precision)" :default 0.0))
  (`/Game/VRGK/Blueprints/Player/GamePawns/BP_VRPhysicsPawn.CurrentGroundComponent` (`self.PhysicsPawnParent`)
    (:`then`
      (set `local.GroundDot` (`KismetMathLibrary.Dot_VectorVector` (`.ImpactNormal` (`GameplayStatics.BreakHitResult` (`self.LastLocomotionGroundHitResult`))) (`self.GetActorUpVector`)))
      (`|ExecutionSequence`
        (:`then_0`
          ;[1 1 1] Prepare the PhysMats that are needed
          (if (and (> (`local.GroundDot`) 0.8) (< (`KismetMathLibrary.VSize` (`self.GetVelocity`)) (`self.StrongFrictionVelocityThreshold`)))
            (set `local.RecommendedStrong` (`self.LocomotionPhysMatStrong`))
            (set `local.RecommendedWeak` (`self.LocomotionPhysMatNormal`))
            (set `local.TargetWeakChangeSpeed` 0.1)
            (elif (> (`local.GroundDot`) 0.7)
              (set `local.RecommendedStrong` (`self.LocomotionPhysMatNormal`))
              (set `local.RecommendedWeak` (`self.LocomotionPhysMatWeak`))
              (set `local.TargetWeakChangeSpeed` 0.0)
              (else
                (return (`self.LocomotionPhysMatWeak`) 0.1)))))
        (:`then_1`
          ;[1 1 1] Calculate if strong or weak PhysMat is chosen.
          (if (and (`/Game/VRGK/Blueprints/Player/PlayerCore/BP_VRGamePawn.Is VR Player Moving With Input` (`self.PhysicsPawnParent`)) (`/Game/VRGK/Blueprints/Player/PlayerCore/BP_VRGamePawn.IsPawnTouchingGround` (`self.PhysicsPawnParent`)))
            (if (`self.FenderSphereIsColliding`)
              _
              (else
                (return (`local.RecommendedStrong`) 0.0))))
          (return (`local.RecommendedWeak`) (`local.TargetWeakChangeSpeed`)))))
    (:`else`
      (return (`self.LocomotionPhysMatWeak`) 0.1) ; If there is no stable ground, just use the weakest Friction PhysMat.
    )))

(fn `ManualSetupConstraint`
  (params (`Target Constraint` :type "PhysicsConstraintComponent Object Reference") (`Child Component` :type "PrimitiveComponent Object Reference") (`Parent Component` :type "PrimitiveComponent Object Reference") (`Child Frame 1` :type "Transform Structure") (`Parent Frame 2` :type "Transform Structure"))
  (`PhysicsConstraintComponent.SetConstrainedComponents` (`local.Target Constraint`) (`local.Child Component`) "None" (`local.Parent Component`) "None")
  (`PhysicsConstraintComponent.SetConstraintReferenceFrame` (`local.Target Constraint`) "Frame1" (`local.Child Frame 1`))
  (`PhysicsConstraintComponent.SetConstraintReferenceFrame` (`local.Target Constraint`) "Frame2" (`local.Parent Frame 2`)))

(fn `ResetPhysicsRigLinearDampingDefaults`
  (`self.SetPhysicsRigLinearDamping` 0.01))

(fn `SetPhysicsRigCollisionProfile`
  (params (InCollisionProfileName :type Name) (bUpdateOverlaps :type Boolean :default true))
  (`PrimitiveComponent.SetCollisionProfileName` (`self.FenderSphere`) InCollisionProfileName bUpdateOverlaps)
  (`PrimitiveComponent.SetCollisionProfileName` (`self.BodyCapsule`) InCollisionProfileName bUpdateOverlaps)
  (`PrimitiveComponent.SetCollisionProfileName` (`self.HeadSphere`) InCollisionProfileName bUpdateOverlaps)
  (`PrimitiveComponent.SetCollisionProfileName` (`self.LocomotionSphere`) InCollisionProfileName bUpdateOverlaps))

(fn `SetPhysicsRigGravityEnabled`
  (params (Enabled :type Boolean))
  (bind _output_get (set `self.IsGravityEnabled` Enabled))
  (`PrimitiveComponent.SetEnableGravity` (`self.FenderSphere`) _output_get)
  (`PrimitiveComponent.SetEnableGravity` (`self.BodyCapsule`) _output_get)
  (`PrimitiveComponent.SetEnableGravity` (`self.HeadSphere`) _output_get)
  (`PrimitiveComponent.SetEnableGravity` (`self.LocomotionSphere`) _output_get))

(fn `SetPhysicsRigLinearDamping`
  (params (`New Value` :type "Float (double-precision)"))
  (`PrimitiveComponent.SetLinearDamping` (`self.FenderSphere`) `New Value`)
  (`PrimitiveComponent.SetLinearDamping` (`self.LocomotionSphere`) `New Value`)
  (`PrimitiveComponent.SetLinearDamping` (`self.BodyCapsule`) `New Value`)
  (`PrimitiveComponent.SetLinearDamping` (`self.HeadSphere`) `New Value`))

(fn `SetPhysicsRigWorldScale`
  (params (`New Scale` :type "Float (double-precision)"))
  (`|ExecutionSequence`
    (:`then_0`
      (`SceneComponent.SetWorldScale3D` (`self.FenderSphere`) (`KismetMathLibrary.Conv_DoubleToVector` (`local.New Scale`)))
      (`SceneComponent.SetWorldScale3D` (`self.BodyCapsule`) (`KismetMathLibrary.Conv_DoubleToVector` (`local.New Scale`)))
      (`SceneComponent.SetWorldScale3D` (`self.HeadSphere`) (`KismetMathLibrary.Conv_DoubleToVector` (`local.New Scale`)))
      (`SceneComponent.SetWorldScale3D` (`self.LocomotionSphere`) (`KismetMathLibrary.Conv_DoubleToVector` (`local.New Scale`)))
      (`PrimitiveComponent.SetMassScale` (`self.FenderSphere`) "None" (`local.New Scale`))
      (`PrimitiveComponent.SetMassScale` (`self.LocomotionSphere`) "None" (`local.New Scale`))
      (`PrimitiveComponent.SetMassScale` (`self.BodyCapsule`) "None" (`local.New Scale`))
      (`PrimitiveComponent.SetMassScale` (`self.HeadSphere`) "None" (`local.New Scale`)))
    (:`then_1`
      (`self.UpdateRigBodyConstraintFrames`)
      (`self.SetRigMaximumHeight` (`self.MaximumRigHeight`)))))

(fn `SetRigMaximumHeight`
  (params (MaxHeight :type "Float (double-precision)"))
  (set `self.MaximumRigHeight` MaxHeight)
  (`PhysicsConstraintComponent.SetLinearZLimit` (`self.HeadSphereConstraint`) "LCM_Limited" (* (`self.Calculate Adjusted Head Height Clamped` (`self.MaximumRigHeight`)) (`/Game/VRGK/Blueprints/Player/PlayerCore/BP_VRGamePawn.GetVRPawnWorldScale` (`self.PhysicsPawnParent`)))))

(fn `SetRigPrimitiveConstraintsEnabled`
  (params (Enabled :type Boolean))
  (`PrimitiveComponent.SetConstraintMode` (`self.FenderSphere`) (select `bool` Enabled :`true` "Default" :!type "EDOFMode Enum")))

(fn `SetRigTargetHeight`
  (params (`New Height` :type "Float (double-precision)"))
  (set `self.TargetRigHeight` `New Height`))

(fn `StopAllPhysicsVelocity`
  (`PrimitiveComponent.SetAllPhysicsLinearVelocity` (`self.FenderSphere`) (0.0 0.0 0.0) false)
  (`PrimitiveComponent.SetAllPhysicsLinearVelocity` (`self.LocomotionSphere`) (0.0 0.0 0.0) false)
  (`PrimitiveComponent.SetAllPhysicsLinearVelocity` (`self.BodyCapsule`) (0.0 0.0 0.0) false)
  (`PrimitiveComponent.SetAllPhysicsLinearVelocity` (`self.HeadSphere`) (0.0 0.0 0.0) false)
  (`PrimitiveComponent.SetAllPhysicsAngularVelocityInDegrees` (`self.FenderSphere`) (0.0 0.0 0.0) false)
  (`PrimitiveComponent.SetAllPhysicsAngularVelocityInDegrees` (`self.LocomotionSphere`) (0.0 0.0 0.0) false)
  (`PrimitiveComponent.SetAllPhysicsAngularVelocityInDegrees` (`self.BodyCapsule`) (0.0 0.0 0.0) false)
  (`PrimitiveComponent.SetAllPhysicsAngularVelocityInDegrees` (`self.HeadSphere`) (0.0 0.0 0.0) false))

(fn `UserConstructionScript`)