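; Base component for hand interaction area presets in the VRGK hand interaction system, meant to be subclassed.
; Its override event copies flip, Z-axis-only rotation and offset axis settings onto the given interaction component, then destroys itself.
; The maximum area offset comes from GetAreaOffsetValue, which returns zero in this base.
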(event `Do Hand Interaction Preset Overrides`
  (params (`Interaction Component` :type "/Game/VRGK/Blueprints/Components/HandInteraction/BPC_HandInteraction Object Reference"))
  (`|ExecutionSequence`
    (:`then_0`
      (set `/Game/VRGK/Blueprints/Components/HandInteraction/BPC_HandInteraction.AllowFlip` (`self.Allow Flip`) `Interaction Component`)
      (set `/Game/VRGK/Blueprints/Components/HandInteraction/BPC_HandInteraction.Allow Rotation (Z-Axis Only)` (`self.Allow Rotation`) `Interaction Component`)
      (set `/Game/VRGK/Blueprints/Components/HandInteraction/BPC_HandInteraction.AreaOffsetAxis` (`self.Area Offset Axis`) `Interaction Component`)
      (set `/Game/VRGK/Blueprints/Components/HandInteraction/BPC_HandInteraction.MaxAreaOffset` (`self.GetAreaOffsetValue`) `Interaction Component`))
    (:`then_1`
      (`self.K2_DestroyComponent`))))

(fn `GetAreaOffsetValue`
  (returns (ReturnValue :type "Float (double-precision)"))
  (return 0.0))