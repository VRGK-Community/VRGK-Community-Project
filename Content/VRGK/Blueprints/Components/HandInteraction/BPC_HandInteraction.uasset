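; Hand interaction component that makes its parent primitive a grab point for VR hands, with hand filtering, distance checks and optional multi-hand grabs.
; On BeginPlay it caches poses from child hand positioners, optionally mirrored, and applies any child area preset.
; GetAttachPosition adapts that pose to the hand through Z rotation, flipping and clamped axis offset.
; It tracks hands and relays grab, trigger and button events, leaving physical attachment to the VRHand Blueprints.
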(event `self.ReceiveBeginPlay`
  ;[1 1 1] BeginPlay / Setup
  (bind _asprimitive_component (cast `PrimitiveComponent` (`self.GetAttachParent`)))
  (set `self.ParentPrimitive` _asprimitive_component)
  (`self.Setup Hand Positioner Transforms`)
  (`self.SetupAreaPresetComponent`))

(event `SetGrabbingEnabled`
  (params (Enabled :type Boolean))
  ;[1 1 1] SetGrabbingEnabled
  (set `self.GrabbingEnabled` Enabled))

(event `AttachThisHand`
  (params (`New Hand` :type "/Game/VRGK/Blueprints/Player/Hand/BP_VRHand Object Reference"))
  ;[1 1 1] Attach Hand (Does not actually change the physical attachment, look into the VRHand Blueprints)
  (if (`self.EnableMultiHand`)
    (`KismetArrayLibrary.Array_AddUnique` (`self.AttachHandList`) `New Hand`)
    (else
      (set `self.OwnerHand` `New Hand`)))
  (`self.OnGrab` self))

(event `PlayHapticEffectOnHand`
  (params (HapticEffect :type "HapticFeedbackEffect_Base Object Reference") (Scale :type "Float (double-precision)" :default 1.0))
  (bind _ownerhand (`self.OwnerHand`))
  ;[1 1 1] Haptic Feedback
  (`/Engine/EditorBlueprintResources/StandardMacros.IsValid` _ownerhand
    (:`Is Valid`
      (`/Game/VRGK/Blueprints/Player/Hand/BP_VRHand.PlayHapticEffectFeedback` _ownerhand HapticEffect Scale))))

(event `ReleaseThisHand`
  (params (`Release Hand` :type "/Game/VRGK/Blueprints/Player/Hand/BP_VRHand Object Reference"))
  ;[1 1 1] Release Hand and reset Interactions
  (if (`self.EnableMultiHand`)
    (`KismetArrayLibrary.Array_RemoveItem` (`self.AttachHandList`) `Release Hand`)
    (`self.OnRelease` self :!label _label)
    (else
      (set `self.OwnerHand` null)
      (`|ExecutionSequence`
        (:`then_0`
          (if (`self.IsTriggerPressed`)
            (`self.TriggerRelease`)))
        (:`then_1`
          (if (`self.IsButtonPressed`)
            (`self.ButtonRelease`)))
        (:`then_2`
          (goto _label))))))

(event `UpdateTrigger`
  (params (Strength :type "Float (double-precision)"))
  ;[1 1 1] Trigger Events
  (bind _output_get (set `self.TriggerStrength` (`KismetMathLibrary.SelectFloat` 1.0 Strength (`self.TriggerPressed`))))
  (`self.OnTriggerChange` _output_get))

(event `TriggerPress`
  ;[1 1 1] Trigger Events
  (set `self.TriggerPressed` true)
  (`self.OnTriggerPressed`))

(event `TriggerRelease`
  ;[1 1 1] Trigger Events
  (set `self.TriggerPressed` false)
  (`self.OnTriggerReleased`))

(event `ButtonPress`
  ;[1 1 1] Button Events
  (set `self.ButtonPressed` true)
  (`self.OnButtonPressed`))

(event `ButtonRelease`
  ;[1 1 1] Button Events
  (set `self.ButtonPressed` false)
  (`self.OnButtonReleased`))

(fn `CanNewHandInteract`
  (params (`Test Hand Type` :type "/Game/VRGK/Blueprints/Player/Hand/Enum_HandType Enum" :default "NewEnumerator0") (GrabOffset :type "Transform Structure") (`Hand World T` :type "Transform Structure"))
  (returns (NearTrue :type Boolean) (GeneralTrue :type Boolean) (Distance :type "Float (double-precision)"))
  (locals (TempDistance :type "Float (double-precision)" :default 0.0))
  (bind _graboffset_location (`KismetMathLibrary.BreakTransform` (`local.GrabOffset`)))
  (bind _atlocation (`self.GetAttachPosition` `Test Hand Type` true GrabOffset `Hand World T`))
  (set `local.TempDistance` (`KismetMathLibrary.Vector_Distance` (`KismetMathLibrary.TransformLocation` (`local.Hand World T`) _graboffset_location) (`KismetMathLibrary.TransformLocation` (`self.K2_GetComponentToWorld` (`self.GetAttachParent`)) _atlocation)))
  (switch `/Game/VRGK/Blueprints/Components/HandInteraction/Enum_AllowedHandTypes` (`self.AllowedHands`)
    (:`NewEnumerator0`
      _)
    (:`NewEnumerator1`
      (if (`|EnumEquality` (`local.Test Hand Type`) "NewEnumerator0")
        _
        (else
          (return false false (`local.TempDistance`)))))
    (:`NewEnumerator2`
      (if (`|EnumEquality` (`local.Test Hand Type`) "NewEnumerator1")
        _
        (else
          (return false false (`local.TempDistance`))))))
  (if (not (`self.EnableMultiHand`))
    (`self.OwnerHand`
      (:`then`
        (return false false (`local.TempDistance`)))
      (:`else`
        _)))
  (return (<= (`local.TempDistance`) (`self.MaxDistance`)) true (`local.TempDistance`)))

(fn `Get Attach World Transform`
  (params (HandType :type "/Game/VRGK/Blueprints/Player/Hand/Enum_HandType Enum" :default "NewEnumerator0"))
  (returns (ReturnValue :type "Transform Structure"))
  (return (`/Game/VRGK/Blueprints/BPFL_GlobalFunctions.TransformTransform` (`self.K2_GetComponentToWorld`) (select `/Game/VRGK/Blueprints/Player/Hand/Enum_HandType` (`local.HandType`) :`NewEnumerator0` (`self.RightHandTransform`) :`NewEnumerator1` (`self.LeftHandTransform`)))))

(fn `Get Attached Hand`
  (returns (`VRHand Reference` :type "/Game/VRGK/Blueprints/Player/Hand/BP_VRHand Object Reference"))
  (return (`self.OwnerHand`)))

(fn `Get Hand Positioner Finger Poser Data`
  (params (`Hand Type` :type "/Game/VRGK/Blueprints/Player/Hand/Enum_HandType Enum" :default "NewEnumerator0"))
  (returns (Valid :type Boolean) (StartData :type "/Game/VRGK/Blueprints/Player/Hand/Struct_FingerData Structure") (FingerData :type "/Game/VRGK/Blueprints/Player/Hand/Struct_FingerData Structure"))
  (locals (TempPositioner :type "/Game/VRGK/Blueprints/Components/HandInteraction/BPC_HandPositioner Object Reference"))
  (bind _temppositioner (`local.TempPositioner`))
  (`|ExecutionSequence`
    (:`then_0`
      (switch `/Game/VRGK/Blueprints/Player/Hand/Enum_HandType` (`local.Hand Type`)
        (:`NewEnumerator0`
          (bind _righthandpositioner (`self.RightHandPositioner`)
            (:`then`
              (set `local.TempPositioner` _righthandpositioner))
            (:`else`
              (set `local.TempPositioner` (`self.LeftHandPositioner`)))))
        (:`NewEnumerator1`
          (bind _lefthandpositioner (`self.LeftHandPositioner`)
            (:`then`
              (set `local.TempPositioner` _lefthandpositioner))
            (:`else`
              (set `local.TempPositioner` (`self.RightHandPositioner`)))))))
    (:`then_1`
      (`/Engine/EditorBlueprintResources/StandardMacros.IsValid` (`local.TempPositioner`)
        (:`Is Valid`
          (if (`/Game/VRGK/Blueprints/Components/HandInteraction/BPC_HandPositioner.UseCustomPoser` (`local.TempPositioner`))
            (return true (`/Game/VRGK/Blueprints/Components/HandInteraction/BPC_HandPositioner.StartData` _temppositioner) (`/Game/VRGK/Blueprints/Components/HandInteraction/BPC_HandPositioner.FingerData` _temppositioner))
            (else
              (return false))))
        (:`Is Not Valid`
          (return false))))))

(fn `GetAttachPosition`
  (params (Hand :type "/Game/VRGK/Blueprints/Player/Hand/Enum_HandType Enum" :default "NewEnumerator0") (OnlyLocationCheck :type Boolean) (GrabOffsetTransform :type "Transform Structure") (HandWorldTransform :type "Transform Structure") (`Force Default` :type Boolean))
  (returns (AtLocation :type "Vector Structure") (WithRotation :type "Rotator Structure") (WithGrabOffset :type Boolean))
  (locals (`Base Hand Transform` :type "Transform Structure") (`Target Hand Transform` :type "Transform Structure") (RotationValue :type "Float (double-precision)" :default 0.0))
  (bind _returnvalue (`self.GetRelativeTransform`))
  (bind (_returnvalue_location _returnvalue_rotation) (`KismetMathLibrary.BreakTransform` (`self.K2_GetComponentToWorld`)))
  (bind (_returnvalue_location_2 _returnvalue_rotation_2) (`KismetMathLibrary.BreakTransform` (`self.K2_GetComponentToWorld`)))
  (bind _target_hand_transform (`local.Target Hand Transform`))
  (bind _maxareaoffset (`self.MaxAreaOffset`))
  (bind _graboffsettransform_location (`KismetMathLibrary.BreakTransform` (`local.GrabOffsetTransform`)))
  (bind _graboffsettransform_location_2 (`KismetMathLibrary.BreakTransform` (`local.GrabOffsetTransform`)))
  (bind _allowflip (`self.AllowFlip`))
  (bind _graboffsettransform_location_3 (`KismetMathLibrary.BreakTransform` (`local.GrabOffsetTransform`)))
  (bind (_graboffsettransform_location_4 _graboffsettransform_rotation) (`KismetMathLibrary.BreakTransform` (`local.GrabOffsetTransform`)))
  (bind (_graboffsettransform_location_5 _graboffsettransform_rotation_2) (`KismetMathLibrary.BreakTransform` (`local.GrabOffsetTransform`)))
  (bind _graboffsettransform_location_6 (`KismetMathLibrary.BreakTransform` (`local.GrabOffsetTransform`)))
  (bind (_base_hand_transform_location _base_hand_transform_rotation) (`KismetMathLibrary.BreakTransform` (`local.Base Hand Transform`)))
  (bind _returnvalue_2 (`KismetMathLibrary.MakeTransform` _returnvalue_location _returnvalue_rotation))
  (bind _returnvalue_3 (`KismetMathLibrary.InverseTransformRotation` _returnvalue_2 (`KismetMathLibrary.TransformRotation` (`local.HandWorldTransform`) _graboffsettransform_rotation_2)))
  (bind _rotation (.rotation (`/Game/VRGK/Blueprints/BPFL_GlobalFunctions.RotateTransformByAxis` "NewEnumerator3" (`local.Target Hand Transform`) (`local.RotationValue`))))
  (bind _returnvalue_4 (`KismetMathLibrary.InverseTransformRotation` (`KismetMathLibrary.MakeTransform` _returnvalue_location_2 _returnvalue_rotation_2) (.rotation (`local.HandWorldTransform`))))
  (bind _returnvalue_5 (`KismetMathLibrary.MakeTransform` (.location _target_hand_transform) (`KismetMathLibrary.TransformRotation` _target_hand_transform (select `/Game/VRGK/Blueprints/Player/Hand/Enum_HandType` (`local.Hand`) :`NewEnumerator0` (struct :`Roll` -90.0) :`NewEnumerator1` (struct :`Roll` 90.0) :!type "Rotator Structure"))))
  (bind (_returnvalue_roll _returnvalue_pitch _returnvalue_yaw) (`KismetMathLibrary.BreakRotator` (`KismetMathLibrary.NormalizedDeltaRotator` (`KismetMathLibrary.MakeRotator` 0.0 0.0 (`KismetMathLibrary.DegAtan2` (.y (+ (`KismetMathLibrary.InverseTransformLocation` _returnvalue_2 (`KismetMathLibrary.TransformLocation` (`local.HandWorldTransform`) _graboffsettransform_location_3)) (* (`KismetMathLibrary.SelectVector` (`KismetMathLibrary.GetUpVector` _returnvalue_3) (* (`KismetMathLibrary.GetForwardVector` _returnvalue_3) -1.0) (`KismetMathLibrary.InRange_FloatFloat` (`KismetMathLibrary.Dot_VectorVector` (`KismetMathLibrary.GetUpVector` _base_hand_transform_rotation) (0.0 0.0 1.0)) -0.5 0.5)) 50.0))) (.x (+ (`KismetMathLibrary.InverseTransformLocation` _returnvalue_2 (`KismetMathLibrary.TransformLocation` (`local.HandWorldTransform`) _graboffsettransform_location_3)) (* (`KismetMathLibrary.SelectVector` (`KismetMathLibrary.GetUpVector` _returnvalue_3) (* (`KismetMathLibrary.GetForwardVector` _returnvalue_3) -1.0) (`KismetMathLibrary.InRange_FloatFloat` (`KismetMathLibrary.Dot_VectorVector` (`KismetMathLibrary.GetUpVector` _base_hand_transform_rotation) (0.0 0.0 1.0)) -0.5 0.5)) 50.0))))) (`KismetMathLibrary.MakeRotator` 0.0 0.0 (`KismetMathLibrary.DegAtan2` (.y (`KismetMathLibrary.TransformLocation` (`local.Target Hand Transform`) _graboffsettransform_location_6)) (.x (`KismetMathLibrary.TransformLocation` (`local.Target Hand Transform`) _graboffsettransform_location_6)))))))
  (bind _output_get (set `local.Base Hand Transform` (select `/Game/VRGK/Blueprints/Player/Hand/Enum_HandType` (`local.Hand`) :`NewEnumerator0` (`self.RightHandTransform`) :`NewEnumerator1` (`self.LeftHandTransform`))))
  (set `local.Target Hand Transform` _output_get)
  (`|ExecutionSequence`
    (:`then_0`
      (if (not (`local.Force Default`))
        (`|ExecutionSequence`
          (:`then_0`
            ;[0.4427 0.3101 0.1352] Base Rotation
            (if (`self.Allow Rotation (Z-Axis Only)`) :!label _label
              (set `local.RotationValue` _returnvalue_yaw)
              (else
                (set `local.RotationValue` 0.0))))
          (:`then_1`
            (if (not (`local.OnlyLocationCheck`))
              (switch `/Game/VRGK/Blueprints/Components/HandInteraction/Enum_HandInteractionFixedMirror` (`self.AllowFlip`)
                (:`NewEnumerator1`
                  _)
                (:`NewEnumerator2`
                  _)
                (:`NewEnumerator3`
                  _))
              (if (not (>= (`KismetMathLibrary.Dot_VectorVector` (select `/Game/VRGK/Blueprints/Components/HandInteraction/Enum_HandInteractionFixedMirror` _allowflip :`NewEnumerator1` (`KismetMathLibrary.GetForwardVector` _rotation) :`NewEnumerator2` (`KismetMathLibrary.GetRightVector` _rotation) :`NewEnumerator3` (`KismetMathLibrary.GetUpVector` _rotation)) (select `/Game/VRGK/Blueprints/Components/HandInteraction/Enum_HandInteractionFixedMirror` _allowflip :`NewEnumerator1` (`KismetMathLibrary.GetForwardVector` _returnvalue_4) :`NewEnumerator2` (`KismetMathLibrary.GetRightVector` _returnvalue_4) :`NewEnumerator3` (`KismetMathLibrary.GetUpVector` _returnvalue_4))) 0.0))
                (set `local.Target Hand Transform` (`/Game/VRGK/Blueprints/BPFL_GlobalFunctions.FlipRotateTransformByAxis` (`self.AllowFlip`) (`local.Target Hand Transform`)))
                (set `local.RotationValue` 0.0))))
          (:`then_2`
            (`|ExecutionSequence`
              (:`then_0`
                (if (not (`local.OnlyLocationCheck`))
                  (goto _label)))
              (:`then_1`
                ;[1 1 1] Actually rotate the Target Hand Transform
                (set `local.Target Hand Transform` (`/Game/VRGK/Blueprints/BPFL_GlobalFunctions.RotateTransformByAxis` "NewEnumerator3" (`local.Target Hand Transform`) (`local.RotationValue`))))))
          (:`then_3`
            ;[1 1 1] Positional Offset on Axis
            (set `local.Target Hand Transform` (`KismetMathLibrary.MakeTransform` (+ (.location (`local.Target Hand Transform`)) (`KismetMathLibrary.ClampVectorSize` (* (- (`KismetMathLibrary.InverseTransformLocation` (`self.K2_GetComponentToWorld`) (`KismetMathLibrary.TransformLocation` (`local.HandWorldTransform`) _graboffsettransform_location)) (`KismetMathLibrary.TransformLocation` (`local.Target Hand Transform`) _graboffsettransform_location_2)) (select `/Game/VRGK/Blueprints/Components/HandInteraction/Enum_HandInteractionFixedMirror` (`self.AreaOffsetAxis`) :`NewEnumerator1` (1.0 0.0 0.0) :`NewEnumerator2` (0.0 1.0 0.0) :`NewEnumerator3` (0.0 0.0 1.0) :!type "Vector Structure")) (* _maxareaoffset -1.0) _maxareaoffset)) (.rotation (`local.Target Hand Transform`)) (.scale (`local.Target Hand Transform`))))))))
    (:`then_1`
      (return (`KismetMathLibrary.TransformLocation` _returnvalue (.location (`KismetMathLibrary.MakeTransform` (`KismetMathLibrary.TransformLocation` _returnvalue_5 _graboffsettransform_location_4) (`KismetMathLibrary.TransformRotation` _returnvalue_5 _graboffsettransform_rotation)))) (`KismetMathLibrary.TransformRotation` _returnvalue (.rotation (`KismetMathLibrary.MakeTransform` (`KismetMathLibrary.TransformLocation` _returnvalue_5 _graboffsettransform_location_4) (`KismetMathLibrary.TransformRotation` _returnvalue_5 _graboffsettransform_rotation)))) true))))

(fn `GetHandAnimData`
  (returns (GrabType :type "/Game/VRGK/Blueprints/Player/Hand/Enum_HandGrabTypes Enum") (StretchedCustomAnimation :type "AnimSequenceBase Object Reference") (OpenedCustomAnimation :type "AnimSequenceBase Object Reference") (ClosedCustomAnimation :type "AnimSequenceBase Object Reference"))
  (bind _hand_animation (`self.Hand Animation`)
    (:`then`
      (return "NewEnumerator2" (`/Game/VRGK/Blueprints/Data/BP_HandAnimationDataAsset.Hand Stretched Animation` _hand_animation) (`/Game/VRGK/Blueprints/Data/BP_HandAnimationDataAsset.Hand Opened Animation` _hand_animation) (`/Game/VRGK/Blueprints/Data/BP_HandAnimationDataAsset.Hand Closed Animation` _hand_animation)))
    (:`else`
      (return "NewEnumerator0" null null null))))

(fn `GetHandMeshAttachment`
  (returns (`Attach Mesh to Component` :type "SceneComponent Object Reference") (`Bone Name` :type Name) (KeepRelative :type Boolean))
  (if (`KismetSystemLibrary.DoesImplementInterface` (`self.GetOwner`) "/Game/VRGK/Blueprints/Components/HandInteraction/BPI_HandInteractionOverride.BPI_HandInteractionOverride_C")
    (bind (_attach_to_component _bone_name _keeprelative) (message `/Game/VRGK/Blueprints/Components/HandInteraction/BPI_HandInteractionOverride.GetHandMeshAttachmentOverride` (`self.GetOwner`) self))
    (return _attach_to_component _bone_name _keeprelative)
    (else
      (return null "None" false))))

(fn `GetParentPrimitiveComponent`
  (returns (ParentPrimitive :type "PrimitiveComponent Object Reference"))
  (return (`self.ParentPrimitive`)))

(fn `GetTriggerStrength`
  (returns (Strength :type "Float (double-precision)"))
  (return (`self.TriggerStrength`)))

(fn `Is Grabbing Enabled`
  (returns (Enabled :type Boolean))
  (return (`self.GrabbingEnabled`)))

(fn `IsButtonPressed`
  (returns (True :type Boolean))
  (return (`self.ButtonPressed`)))

(fn `IsGrabbed`
  (returns (True :type Boolean))
  (return (or (`KismetSystemLibrary.IsValid` (`self.OwnerHand`)) (> (`KismetArrayLibrary.Array_Length` (`self.AttachHandList`)) 0))))

(fn `IsTriggerPressed`
  (returns (True :type Boolean))
  (return (`self.TriggerPressed`)))

(fn `SetUnlockedMotion`
  (params (UnlockedMotion :type Boolean) (UnlockedRotation :type Boolean))
  (bind _ownerhand (`self.OwnerHand`)
    (:`then`
      (`/Game/VRGK/Blueprints/Player/Hand/BP_VRHand.SetGrabbingConstraintState` _ownerhand UnlockedMotion UnlockedRotation))
    (:`else`)))

(fn `Setup Hand Positioner Transforms`
  (locals (RightHandAttacher2 :type "/Game/VRGK/Blueprints/Components/HandInteraction/BPC_HandPositioner Object Reference") (LeftHandAttacher2 :type "/Game/VRGK/Blueprints/Components/HandInteraction/BPC_HandPositioner Object Reference"))
  (bind _mirrorhandfixedposition (`self.MirrorHandFixedPosition`))
  (for _array_element (`self.GetChildrenComponents` false)
    (bind _asbpc_hand_positioner (cast `/Game/VRGK/Blueprints/Components/HandInteraction/BPC_HandPositioner` _array_element))
    (switch `/Game/VRGK/Blueprints/Player/Hand/Enum_HandType` (`/Game/VRGK/Blueprints/Components/HandInteraction/BPC_HandPositioner.GetHandType` _asbpc_hand_positioner)
      (:`NewEnumerator0`
        (set `self.RightHandPositioner` _asbpc_hand_positioner))
      (:`NewEnumerator1`
        (set `self.LeftHandPositioner` _asbpc_hand_positioner))))
  (`|ExecutionSequence`
    (:`then_0`
      (bind _righthandpositioner (`self.RightHandPositioner`)
        (:`then`
          (bind _returnvalue (`KismetMathLibrary.MakeTransform` (.location (`self.GetRelativeTransform` _righthandpositioner)) (.rotation (`self.GetRelativeTransform` _righthandpositioner))))
          (set `self.RightHandTransform` _returnvalue)
          (switch `/Game/VRGK/Blueprints/Components/HandInteraction/Enum_HandInteractionFixedMirror` _mirrorhandfixedposition
            (:`NewEnumerator0`
              (bind _lefthandpositioner (`self.LeftHandPositioner`)
                (:`then`
                  (bind (_returnvalue_location _returnvalue_rotation) (`KismetMathLibrary.BreakTransform` (`self.GetRelativeTransform` _lefthandpositioner)))
                  (set `self.LeftHandTransform` (`KismetMathLibrary.MakeTransform` _returnvalue_location _returnvalue_rotation)))
                (:`else`)))
            (:`NewEnumerator1`
              (set `self.LeftHandTransform` (`/Game/VRGK/Blueprints/BPFL_GlobalFunctions.MirrorTransformByAxis` _mirrorhandfixedposition _returnvalue) :!label _label))
            (:`NewEnumerator2`
              (goto _label))
            (:`NewEnumerator3`
              (goto _label))))
        (:`else`)))
    (:`then_1`
      ;[1 0.664 0.4194] Destroy Attachers after Caching Transforms
      (bind _righthandpositioner_2 (`self.RightHandPositioner`)
        (:`then`)
        (:`else`)))
    (:`then_2`
      (bind _lefthandpositioner_2 (`self.LeftHandPositioner`)
        (:`then`)
        (:`else`)))))

(fn `SetupAreaPresetComponent`
  (returns (Success :type Boolean))
  (`/Engine/EditorBlueprintResources/StandardMacros.IsValid` (`self.AreaPresetComponent`)
    (:`Is Valid`
      (return true))
    (:`Is Not Valid`
      (for _array_element (`self.GetChildrenComponents` false)
        (bind _asbpc_hand_interaction_area_preset_base (cast `/Game/VRGK/Blueprints/Components/HandInteraction/PresetComponents/BPC_HandInteractionAreaPresetBase` _array_element))
        (`|ExecutionSequence`
          (:`then_0`
            (break))
          (:`then_1`
            (set `self.AreaPresetComponent` _asbpc_hand_interaction_area_preset_base)
            (`self.UpdatePlacementWithPreset`)
            (return true))))
      (return (`KismetSystemLibrary.IsValid` (`self.AreaPresetComponent`))))))

(fn `TryReleaseCurrentHand`
  (locals (TempHandList :type "Array of /Game/VRGK/Blueprints/Player/Hand/BP_VRHand Object Reference"))
  (if (`self.IsGrabbed`)
    (if (`self.EnableMultiHand`)
      (bind _output_get (set `local.TempHandList` (`self.AttachHandList`)))
      (for _array_element _output_get
        (`/Game/VRGK/Blueprints/Player/Hand/BP_VRHand.Release` _array_element))
      (else
        (bind _ownerhand (`self.OwnerHand`)
          (:`then`
            (`/Game/VRGK/Blueprints/Player/Hand/BP_VRHand.Release` _ownerhand))
          (:`else`))))))

(fn `UpdatePlacementWithPreset`
  (bind _areapresetcomponent (`self.AreaPresetComponent`)
    (:`then`
      (`/Game/VRGK/Blueprints/Components/HandInteraction/PresetComponents/BPC_HandInteractionAreaPresetBase.Do Hand Interaction Preset Overrides` _areapresetcomponent self))
    (:`else`)))