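; BPC_HandGrabUpdater is a VR component that tracks which hands grab its owning object and updates the object's collision to match.
; Registering or unregistering a hand updates the hand array, fires grab or release calls and resets hands' collision tracker hits.
; If enabled, the root primitive swaps between default and grabbed collision profiles.
; An optional owner interface can force the IsColliding checks true, and helpers release all hands or bind hit events.
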(event `RegisterHand`
  (params (VRHand :type "/Game/VRGK/Blueprints/Player/Hand/BP_VRHand Object Reference"))
  ;[1 1 1] Register Hand,  Hand has grabbed this Object.
  (`|ExecutionSequence`
    (:`then_0`
      (if (not (`KismetArrayLibrary.Array_Contains` (`self.GrabHandArray`) VRHand))
        (`KismetArrayLibrary.Array_AddUnique` (`self.GrabHandArray`) VRHand)
        (`self.UpdateCollisionProfileState`)))
    (:`then_1`
      (`self.OnAnyGrab` self)
      (`self.TryResetAllHandsHitEvents`))))

(event `TryResetAllHandsHitEvents`
  ;[1 1 1] Try Reset Hit Events of Hands
  (for _array_element (`self.GrabHandArray`)
    (`/Game/VRGK/Blueprints/Player/Hand/BP_VRHand.Try Reset Both Hands Collision Tracker Hits` _array_element)))

(event `UnregisterHand`
  (params (VRHand :type "/Game/VRGK/Blueprints/Player/Hand/BP_VRHand Object Reference"))
  ;[1 1 1] Unregister Hand, Hand has dropped this Object.
  (`|ExecutionSequence`
    (:`then_0`
      (if (`KismetArrayLibrary.Array_Contains` (`self.GrabHandArray`) VRHand)
        (`KismetArrayLibrary.Array_RemoveItem` (`self.GrabHandArray`) VRHand)
        (`self.UpdateCollisionProfileState`)))
    (:`then_1`
      (`self.OnAnyRelease` self)
      (`self.TryResetAllHandsHitEvents`))))

(event `UpdateCollisionProfileState`
  ;[0.7229 0.3022 1] Update Collision Profile State based on Grabbing or not Grabbing
  (if (`self.UpdateCollisionProfileWhileGrabbed`)
    (`|ExecutionSequence`
      (:`then_0`
        (bind _asprimitive_component (cast `PrimitiveComponent` (`Actor.RootComponent` (`self.GetOwner`)))
          (:`then`
            (`PrimitiveComponent.SetCollisionProfileName` _asprimitive_component (select `bool` (`self.HasHandGrabbing`) :`false` (`self.DefaultCollisionProfile`) :`true` (`self.GrabbedCollisionProfile`)) true))
          (:`CastFailed`
            ;;[1 0.4656 0.4656] Write a Message that there was an error
            (`KismetSystemLibrary.PrintString` "HandGrabCollisionUpdater can't find a Primitive Root Component. Needed to Update Collision Profile."))))
      (:`then_1`
        (`self.OnCollisionUpdate` (`self.HasHandGrabbing`))))))

(fn `GetAttachedHands`
  (returns (`Attached Hands` :type "Array of /Game/VRGK/Blueprints/Player/Hand/BP_VRHand Object Reference"))
  (return (`self.GrabHandArray`)))

(fn `HasHandGrabbing`
  (returns (True :type Boolean))
  (return (> (`KismetArrayLibrary.Array_Length` (`self.GrabHandArray`)) 0)))

(fn `IsColliding`
  (returns (True :type Boolean))
  (if (`KismetSystemLibrary.DoesImplementInterface` (`self.GetOwner`) "/Game/VRGK/Blueprints/Components/GrabCollisionUpdater/BPI_HandGrabCollisionUpdaterOverride.BPI_HandGrabCollisionUpdaterOverride_C")
    (bind _is_colliding (message `/Game/VRGK/Blueprints/Components/GrabCollisionUpdater/BPI_HandGrabCollisionUpdaterOverride.IsForcingHitCollision` (`self.GetOwner`)))
    (return (or _is_colliding (`parent.IsColliding`)))
    (else
      (return (`parent.IsColliding`)))))

(fn `IsStronglyColliding`
  (returns (True :type Boolean))
  (if (`KismetSystemLibrary.DoesImplementInterface` (`self.GetOwner`) "/Game/VRGK/Blueprints/Components/GrabCollisionUpdater/BPI_HandGrabCollisionUpdaterOverride.BPI_HandGrabCollisionUpdaterOverride_C")
    (bind _is_colliding (message `/Game/VRGK/Blueprints/Components/GrabCollisionUpdater/BPI_HandGrabCollisionUpdaterOverride.IsForcingHitCollision` (`self.GetOwner`)))
    (return (or _is_colliding (`parent.IsStronglyColliding`)))
    (else
      (return (`parent.IsStronglyColliding`)))))

(fn `TryBindAllHitEventsToHand`
  (params (Hand :type "/Game/VRGK/Blueprints/Player/Hand/BP_VRHand Object Reference"))
  (`/Game/VRGK/Blueprints/Player/Hand/BP_VRHand.TryBindCollisionTrackerHits` Hand))

(fn `TryReleaseAllGrabbedHands`
  (locals (TempHandList :type "Array of /Game/VRGK/Blueprints/Player/Hand/BP_VRHand Object Reference"))
  (bind _output_get (set `local.TempHandList` (`self.GrabHandArray`)))
  (for _array_element _output_get
    (`/Game/VRGK/Blueprints/Player/Hand/BP_VRHand.Release` _array_element)))

(fn `TryUnbindAllHitEventsFromHand`
  (params (Hand :type "/Game/VRGK/Blueprints/Player/Hand/BP_VRHand Object Reference"))
  (`/Game/VRGK/Blueprints/Player/Hand/BP_VRHand.TryUnbindCollisionTrackerHits` Hand))