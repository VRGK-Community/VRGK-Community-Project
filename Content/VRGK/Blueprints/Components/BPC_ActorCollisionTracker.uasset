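; Actor component that tracks whether its owner and other bound actors, including welded hierarchies, are colliding or strongly colliding.
; Hit events skip bound or ignored actors, including those of an optional second tracker, while force-hit actors bypass impulse checks.
; Strong hits compare impulse to a threshold, switched by a soft-collision tag.
; Once-per-frame gates limit dispatchers, and retriggerable delays clear states, recording when strong contact ended.
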(event `self.ReceiveBeginPlay`
  ;[0.229 1 0.582 1 32] Begin Play
  (if (`self.AutomaticHitSetup`)
    (`self.BindActorToHitEvent` (`self.GetOwner`))))

(event `BindActorToHitEvent`
  (params (Target :type "Actor Object Reference"))
  ;[1 1 1] Bind / Unbind Actors to this Tracker
  (if (not (`KismetArrayLibrary.Array_Contains` (`self.BoundActorList`) Target))
    (add `Actor.OnActorHit` Target (`|CreateDelegate` :!event `OnParentActorHit`))
    (`KismetArrayLibrary.Array_AddUnique` (`self.BoundActorList`) Target)))

(event `AddForceHitActor`
  (params (ActorToUse :type "Actor Object Reference"))
  ;[0.7326 0.3536 1] Force Hit Actors. These ignore the collision checks and activate the Colliding and Strongly Colliding values instantly.
  (`KismetArrayLibrary.Array_AddUnique` (`self.ForceHitActorList`) ActorToUse))

(event `RemoveForceHitActor`
  (params (ActorToUse :type "Actor Object Reference"))
  ;[0.7326 0.3536 1] Force Hit Actors. These ignore the collision checks and activate the Colliding and Strongly Colliding values instantly.
  (`KismetArrayLibrary.Array_RemoveItem` (`self.ForceHitActorList`) ActorToUse))

(event `UnbindActorFromHitEvent`
  (params (Target :type "Actor Object Reference"))
  ;[1 1 1] Bind / Unbind Actors to this Tracker
  (remove `Actor.OnActorHit` Target (`|CreateDelegate` :!event `OnParentActorHit`))
  (`KismetArrayLibrary.Array_RemoveItem` (`self.BoundActorList`) Target))

(event `AddIgnoreHitActor`
  (params (ActorToUse :type "Actor Object Reference"))
  ;[1 0.6087 0.2627] Ignore Hit Actors. These ignore the collision hit checks.
  (`KismetArrayLibrary.Array_AddUnique` (`self.IgnoreHitActorList`) ActorToUse))

(event `RemoveIgnoreHitActor`
  (params (ActorToUse :type "Actor Object Reference"))
  ;[1 0.6087 0.2627] Ignore Hit Actors. These ignore the collision hit checks.
  (`KismetArrayLibrary.Array_RemoveItem` (`self.IgnoreHitActorList`) ActorToUse))

(event `OnParentActorHit`
  (params (SelfActor :type "Actor Object Reference") (OtherActor :type "Actor Object Reference") (NormalImpulse :type "Vector Structure") (Hit :type "HitResult Structure (by ref)"))
  ;[1 0.4448 0.407] Actor Hit Events
  ;;[0.5052 0.04628 0.05131] Check for Ignored Hits.
  (`|ExecutionSequence`
    (:`then_0`
      (bind _doignore (`self.CheckIfActorCanBeIgnored` OtherActor))
      (if (not _doignore)
        ;;[1 0.3024 0.7932] Check for Forced Hits
        (if (`KismetArrayLibrary.Array_Contains` (`self.ForceHitActorList`) OtherActor)
          ;;[1 1 1] Fail Safe, if the hit object happens to be the same as the Owner.
          (`self.OnManualCollision`)
          (`self.OnManualStrongCollision`)
          (else
            (`self.TryDoStrongCollision` NormalImpulse Hit)))))
    (:`then_1`
      (`self.TryDoNormalCollision`))))

(event `TryDoNormalCollision`
  ;[1 0.4448 0.407] Actor Hit Events
  ;;[1 1 1] Check if Any Collision has happened in current Frame.
  (`/Engine/EditorBlueprintResources/StandardMacros.DoOnce` false :!label _label
    (:`Completed`
      (`|ExecutionSequence`
        (:`then_0`
          (set `self.ObjectIsColliding` true)
          (`self.OnObjectIsColliding`)
          (`KismetSystemLibrary.RetriggerableDelay` (`self.CollisionResetDelay`) :!label _label_2)
          (if (`self.ObjectIsColliding`)
            (set `self.ObjectIsColliding` false)))
        (:`then_1`
          (`KismetSystemLibrary.Delay` 0.0)
          (goto _label :!via `Reset`))))))

(event `OnManualCollision`
  ;[1 0.4448 0.407] Actor Hit Events
  ;;[1 1 1] Check if Any Collision has happened in current Frame.
  (set `self.ObjectIsColliding` true)
  (goto _label_2))

(event `TryDoStrongCollision`
  (params (`Normal Impulse` :type "Vector Structure") (`Hit Result` :type "HitResult Structure"))
  (bind (_bblockinghit _binitialoverlap _time _distance _location _impactpoint _normal _impactnormal _physmat _hitactor _hitcomponent) (`GameplayStatics.BreakHitResult` `Hit Result`))
  (bind _softstrongcollisiontag (`self.SoftStrongCollisionTag`))
  ;[1 0.4638 0.02823] Check for Strong Collisions.
  (`/Engine/EditorBlueprintResources/StandardMacros.DoOnce` false :!label _label_3
    (:`Completed`
      (`|ExecutionSequence`
        (:`then_0`
          (if (> (`KismetMathLibrary.VSize` `Normal Impulse`) (`KismetMathLibrary.SelectFloat` (`self.SoftStrongHitThreshold`) (`self.StrongHitThreshold`) (or (`Actor.ActorHasTag` _hitactor _softstrongcollisiontag) (`self.ComponentHasTag` _hitcomponent _softstrongcollisiontag))))
            (`|ExecutionSequence`
              (:`then_0`
                (set `self.ObjectIsStronglyColliding` true))
              (:`then_1`
                (`KismetSystemLibrary.Delay` 0.0)
                (goto _label_3 :!via `Reset`)))
            (else
              (goto _label_3 :!via `Reset`))))
        (:`then_1`
          (`KismetSystemLibrary.RetriggerableDelay` (`self.StrongCollisionResetDelay`) :!label _label_4)
          (if (`self.ObjectIsStronglyColliding`)
            (set `self.ObjectIsStronglyColliding` false)
            (set `self.StrongCollisionEndingTime` (`Actor.GetGameTimeSinceCreation` (`self.GetOwner`)))))
        (:`then_2`
          (`self.FireObjectIsStronglyCollidingDispatcher`))))))

(event `FireObjectIsStronglyCollidingDispatcher`
  ;[1 0.4638 0.02823] Check for Strong Collisions.
  ;;[1 0.6498 0.8459] Callback for Strongly Colliding with Event Dispatchers
  (`/Engine/EditorBlueprintResources/StandardMacros.DoOnce` false :!label _label_5
    (:`Completed`
      (`|ExecutionSequence`
        (:`then_0`
          (if (`self.ObjectIsStronglyColliding`)
            (`self.OnObjectIsStronglyColliding`)))
        (:`then_1`
          (`KismetSystemLibrary.Delay` 0.0) ; Wait for next Frame / Only allow once per Frame
          (goto _label_5 :!via `Reset`))))))

(event `OnManualStrongCollision`
  ;[1 0.4638 0.02823] Check for Strong Collisions.
  (`|ExecutionSequence`
    (:`then_0`
      (if (not (`self.ObjectIsStronglyColliding`))
        (set `self.ObjectIsStronglyColliding` true)))
    (:`then_1`
      (goto _label_4))
    (:`then_2`
      (`self.FireObjectIsStronglyCollidingDispatcher`))))

(fn `CheckIfActorCanBeIgnored`
  (params (`Other Actor` :type "Actor Object Reference"))
  (returns (DoIgnore :type Boolean))
  (bind _other_actor (`local.Other Actor`))
  (`|ExecutionSequence`
    (:`then_0`
      (bind _trackertoignore (`self.TrackerToIgnore`)
        (:`then`
          (if (or (`KismetArrayLibrary.Array_Contains` (`/Game/VRGK/Blueprints/Components/BPC_ActorCollisionTracker.BoundActorList` _trackertoignore) (`local.Other Actor`)) (`KismetArrayLibrary.Array_Contains` (`/Game/VRGK/Blueprints/Components/BPC_ActorCollisionTracker.IgnoreHitActorList` _trackertoignore) (`local.Other Actor`)))
            (return true)))
        (:`else`)))
    (:`then_1`
      (if (or (`KismetArrayLibrary.Array_Contains` (`self.BoundActorList`) _other_actor) (`KismetArrayLibrary.Array_Contains` (`self.IgnoreHitActorList`) _other_actor))
        (return true)))
    (:`then_2`
      (return false))))

(fn `IsColliding`
  (returns (True :type Boolean))
  (return (`self.ObjectIsColliding`)))

(fn `IsStronglyColliding`
  (returns (True :type Boolean))
  (return (`self.ObjectIsStronglyColliding`)))

(fn `TimeSinceLastStrongCollision`
  (returns (`Time in Seconds` :type "Float (double-precision)"))
  (return (`KismetMathLibrary.SelectFloat` 0.0 (- (`Actor.GetGameTimeSinceCreation` (`self.GetOwner`)) (`self.StrongCollisionEndingTime`)) (`self.IsStronglyColliding`))))

(fn `Try Bind All Hit Events From Welded Primitive Component`
  (params (Primitive :type "PrimitiveComponent Object Reference") (`Primitive Bone` :type Name) (ExcludeActors :type "Array of Actor Object Reference"))
  (locals (PrimRoot :type "PrimitiveComponent Object Reference"))
  (`|ExecutionSequence`
    (:`then_0`
      (bind (_hasphysicsroot _physics_root) (`/Game/VRGK/Blueprints/BPFL_PhysicsObjects.GetPhysicsRoot` (`local.Primitive`) (`local.Primitive Bone`)))
      (`/Engine/EditorBlueprintResources/StandardMacros.IsValid` _physics_root
        (:`Is Valid`
          (set `local.PrimRoot` _physics_root))
        (:`Is Not Valid`
          (set `local.PrimRoot` (`local.Primitive`)))))
    (:`then_1`
      (`self.BindActorToHitEvent` (`self.GetOwner` (`local.PrimRoot`)))
      (for _array_element (`SceneComponent.GetChildrenComponents` (`local.PrimRoot`) true)
        (bind _asprimitive_component (cast `PrimitiveComponent` _array_element))
        (bind _returnvalue (`self.GetOwner` _asprimitive_component))
        (if (not (`KismetArrayLibrary.Array_Contains` (`local.ExcludeActors`) _returnvalue))
          (`self.BindActorToHitEvent` _returnvalue))))))

(fn `Unbind All Hit Events`
  (params (`Ignore Owner` :type Boolean))
  (locals (TempActorList :type "Array of Actor Object Reference"))
  (bind _output_get (set `local.TempActorList` (`self.BoundActorList`)))
  (for _array_element _output_get
    (if (`local.Ignore Owner`)
      (if (!= (`self.GetOwner`) _array_element)
        (`self.UnbindActorFromHitEvent` _array_element :!label _label))
      (else
        (goto _label)))))