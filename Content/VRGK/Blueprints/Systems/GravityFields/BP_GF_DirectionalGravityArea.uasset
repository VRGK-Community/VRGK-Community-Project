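; Directional gravity field actor that defines a box-shaped area with uniform gravity along its local down axis.
; GetGravityAreaDirection transforms a downward rotation by the actor's transform and returns it with the area's priority and strength.
; IsInRange converts a location to local space and tests it against fixed box bounds sitting above the origin, so actor rotation and scale shape the volume without overlap events.
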(fn `GetGravityAreaDirection`
  (params (AtLocation :type "Vector Structure"))
  (returns (ToRotation :type "Rotator Structure") (Priority :type Integer) (Strength :type "Float (double-precision)"))
  (return (`KismetMathLibrary.TransformRotation` (`self.GetTransform`) (`KismetMathLibrary.FindLookAtRotation` (0.0 0.0 0.0) (0.0 0.0 -1.0))) (`self.Priority`) (`self.GravityStrength`)))

(fn `IsInRange`
  (params (AtLocation :type "Vector Structure"))
  (returns (InRange :type Boolean))
  (bind (_returnvalue_x _returnvalue_y _returnvalue_z) (`KismetMathLibrary.BreakVector` (`KismetMathLibrary.InverseTransformLocation` (`self.GetTransform`) AtLocation)))
  (return (and (`KismetMathLibrary.InRange_FloatFloat` _returnvalue_x -50.0 50.0 false false) (`KismetMathLibrary.InRange_FloatFloat` _returnvalue_y -50.0 50.0 false false) (`KismetMathLibrary.InRange_FloatFloat` _returnvalue_z 0.0 100.0 false false))))

(fn `UserConstructionScript`
  (`parent.UserConstructionScript`))