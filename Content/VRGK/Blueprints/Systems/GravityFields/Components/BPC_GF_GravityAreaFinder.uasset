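; Actor component that finds the owner's gravity from overlapping gravity areas and smoothly turns toward it each tick.
; It samples areas at the owner's GravityCenter components, or actor location if none; highest priority wins and equal priorities blend.
; Results from multiple centers blend subject to a rotation threshold.
; Direction and strength feed an optional CustomGravity component and an update event, with the last target direction held outside areas.
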(event `self.ReceiveBeginPlay`
  (`self.SetAreaFinderEnabled` (`self.IsActivated`))
  (`|ExecutionSequence`
    (:`then_0`
      ;[1 1 1] Setup the BPC_GF_CustomGravity component if available
      (if (`self.UseCustomGravityComponent`)
        (set `self.GravityComponent` (`Actor.GetComponentByClass` (`self.GetOwner`) "/Game/VRGK/Blueprints/Systems/GravityFields/Components/BPC_GF_CustomGravity.BPC_GF_CustomGravity_C"))))
    (:`then_1`
      ;[1 1 1] Searches for additional Gravity Centers
      (set `self.GravityCenters` (`Actor.K2_GetComponentsByClass` (`self.GetOwner`) "/Game/VRGK/Blueprints/Systems/GravityFields/Components/BPC_GF_GravityCenter.BPC_GF_GravityCenter_C")))
    (:`then_2`
      ;[1 1 1] Calculate the Gravity Direction on BeginPlay
      (bind (_found _gravityoutput _strengthoutput) (`self.CalculateCombinedCurrentDirection`))
      (if _found
        (bind _output_get (set `self.NewGravityRotation` _gravityoutput))
        (bind _output_get_2 (set `self.CurGravityRotation` _output_get))
        (set `self.CurrentGravity` (`KismetMathLibrary.GetForwardVector` _output_get_2))
        (set `self.CurGravityStrength` _strengthoutput)
        (else
          (bind _output_get_3 (set `self.CurrentGravity` (`self.DefaultGravity`)))
          (bind _output_get_4 (set `self.NewGravityRotation` (`KismetMathLibrary.MakeRotationFromAxes` _output_get_3)))
          (set `self.CurGravityRotation` _output_get_4)
          (set `self.CurGravityStrength` 1.0)))
      (`self.UpdateGravity`))))

(event `self.ReceiveTick`
  (params (DeltaSeconds :type "Float (single-precision)"))
  (`self.UpdateGravity`))

(event `SetAreaFinderEnabled`
  (params (Enabled :type Boolean))
  (bind _output_get (set `self.IsActivated` Enabled))
  (`self.SetComponentTickEnabled` _output_get))

(event `UpdateGravity`
  (bind _gravitycomponent (`self.GravityComponent`))
  (bind _returnvalue (`Actor.K2_GetActorLocation` (`self.GetOwner`)))
  ;[1 1 1] Finds all overlapping Gravity Areas and updates the current Rotation and Direction
  (bind (_found _gravityoutput _strengthoutput) (`self.CalculateCombinedCurrentDirection`))
  (set `self.NewGravityRotation` _gravityoutput)
  (set `self.CurGravityStrength` _strengthoutput)
  (`self.UpdateGravityRotation`)
  (`|ExecutionSequence`
    (:`then_0`
      ;[1 1 1] Changes the BPC_GF_CustomGravity component if available
      (`/Engine/EditorBlueprintResources/StandardMacros.IsValid` _gravitycomponent
        (:`Is Valid`
          (set `/Game/VRGK/Blueprints/Systems/GravityFields/Components/BPC_GF_CustomGravity.GravityDirection` (`self.CurrentGravity`) _gravitycomponent)
          (set `/Game/VRGK/Blueprints/Systems/GravityFields/Components/BPC_GF_CustomGravity.GravityMultiplier` (`self.CurGravityStrength`) _gravitycomponent))))
    (:`then_1`
      ;[1 1 1] Debug
      (if (`self.DrawDebug`)
        (`KismetSystemLibrary.DrawDebugArrow` _returnvalue (+ _returnvalue (* (`self.CurrentGravity`) 100.0)) 30.0 (struct :`R` 0.456411 :`B` 0.552012 :`A` 1.0) 0.0 5.0)))
    (:`then_2`
      (if (`self.IsActivated`)
        (`self.OnGravityUpdate` (`self.CurrentGravity`) (`self.CurGravityStrength`))))))

(event `UpdateGravityRotation`
  ;[1 1 1] Updates the current Gravity Rotation and Direction
  (bind _output_get (set `self.CurGravityRotation` (`KismetMathLibrary.RLerp` (`self.CurGravityRotation`) (`self.NewGravityRotation`) (`KismetMathLibrary.FClamp` (* (`GameplayStatics.GetWorldDeltaSeconds`) (`self.LerpSpeed`))) true)))
  (set `self.CurrentGravity` (`KismetMathLibrary.GetForwardVector` _output_get)))

(fn `CalculateCombinedCurrentDirection`
  (returns (Found :type Boolean) (GravityOutput :type "Rotator Structure") (StrengthOutput :type "Float (double-precision)"))
  (locals (OneValid :type Boolean) (TempGravity :type "Rotator Structure" :default (struct)) (TempStrength :type "Float (double-precision)" :default 0.0))
  (bind _returnvalue (`self.GetGravityLocations`))
  (if (== (`KismetArrayLibrary.Array_Length` _returnvalue) 1)
    (bind (_found _gravityoutput _strengthoutput) (`self.CalculateCurrentDirection` (`|GetArrayItem` _returnvalue)))
    (return _found _gravityoutput _strengthoutput)
    (else
      (for (_array_element _array_index) _returnvalue
        (bind (_found_2 _gravityoutput_2 _strengthoutput_2) (`self.CalculateCurrentDirection` _array_element))
        (if (== _array_index 0)
          (set `local.TempGravity` _gravityoutput_2)
          (set `local.TempStrength` _strengthoutput_2)
          (if _found_2
            (set `local.OneValid` true))
          (elif (not (`local.OneValid`))
            (if _found_2
              (set `local.OneValid` true)
              (set `local.TempGravity` _gravityoutput_2)
              (set `local.TempStrength` _strengthoutput_2))
            (elif _found_2
              (bind (_length _returnvalue_2) (`/Game/VRGK/Blueprints/Systems/GravityFields/BPFL_GravityFields.RotationThreshold` (`local.TempGravity`) _gravityoutput_2 (`self.CombinedRotThreshold`)))
              (set `local.TempGravity` (`KismetMathLibrary.SelectRotator` (`KismetMathLibrary.RLerp` (`local.TempGravity`) _gravityoutput_2 0.5 true) (`local.TempGravity`) _returnvalue_2))
              (set `local.TempStrength` (`KismetMathLibrary.SelectFloat` (`KismetMathLibrary.Lerp` (`local.TempStrength`) _strengthoutput_2 0.5) (`local.TempStrength`) _returnvalue_2))))))
      (return (`local.OneValid`) (`local.TempGravity`) (`local.TempStrength`)))))

(fn `CalculateCurrentDirection`
  (params (AtLocation :type "Vector Structure"))
  (returns (Found :type Boolean) (GravityOutput :type "Rotator Structure") (StrengthOutput :type "Float (double-precision)"))
  (locals (TempLocation :type "Vector Structure") (TempGravityRotation :type "Rotator Structure") (TempPriority :type Integer) (FirstAreaDone :type Boolean) (TempStrength :type "Float (double-precision)" :default 1.0))
  (bind _temppriority (`local.TempPriority`))
  (bind _overlappingactors (`Actor.GetOverlappingActors` (`self.GetOwner`) "/Game/VRGK/Blueprints/Systems/GravityFields/BP_GF_GravityAreaBase.BP_GF_GravityAreaBase_C"))
  (set `local.TempLocation` AtLocation)
  (if (> (`KismetArrayLibrary.Array_Length` _overlappingactors) 0)
    (for _array_element _overlappingactors
      (bind _inrange (message `/Game/VRGK/Blueprints/Systems/GravityFields/BPI_GF_GravityArea.IsInRange` _array_element (`local.TempLocation`)))
      (if _inrange
        (bind (_torotation _priority _strength) (message `/Game/VRGK/Blueprints/Systems/GravityFields/BPI_GF_GravityArea.GetGravityAreaDirection` _array_element (`local.TempLocation`)))
        (if (not (`local.FirstAreaDone`))
          (set `local.FirstAreaDone` true)
          (set `local.TempGravityRotation` _torotation :!label _label)
          (set `local.TempPriority` _priority)
          (set `local.TempStrength` _strength)
          (elif (== _priority _temppriority)
            (set `local.TempGravityRotation` (`KismetMathLibrary.RLerp` (`local.TempGravityRotation`) _torotation 0.5 true))
            (set `local.TempStrength` (`KismetMathLibrary.Lerp` (`local.TempStrength`) _strength 0.5))
            (elif (> _priority _temppriority)
              (goto _label))))))
    (if (`local.FirstAreaDone`)
      (return true (`local.TempGravityRotation`) (`local.TempStrength`))
      (else
        _)))
  (return false (`self.NewGravityRotation`) (`local.TempStrength`)))

(fn `GetGravity`
  (returns (`Gravity Direction` :type "Vector Structure") (`Gravity Strength` :type "Float (double-precision)"))
  (return (`self.CurrentGravity`) (`self.CurGravityStrength`)))

(fn `GetGravityLocations`
  (returns (ReturnValue :type "Array of Vector Structure"))
  (locals (TempLocations :type "Array of Vector Structure"))
  (if (> (`KismetArrayLibrary.Array_Length` (`self.GravityCenters`)) 0)
    (for _array_element (`self.GravityCenters`)
      (`KismetArrayLibrary.Array_Add` (`local.TempLocations`) (`SceneComponent.K2_GetComponentLocation` _array_element)))
    (return (`local.TempLocations`))
    (else
      (return (`|MakeArray` (`Actor.K2_GetActorLocation` (`self.GetOwner`)))))))