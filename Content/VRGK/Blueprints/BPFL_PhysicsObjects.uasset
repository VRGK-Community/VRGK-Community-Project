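; Blueprint function library of helpers for physics-simulated objects in VRGK.
; AttachObjectToPhysicalParent enables physics on a child actor's root and attaches it to the simulating primitive above its child actor component.
; GetPhysicsRoot climbs a movable component's parent chain to return the last consecutively simulating primitive and bone name.
; TryResetPhysicsSimulation toggles simulation to fix faulty collisions, restoring cached linear and angular velocities afterwards.
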(fn `Attach Object to Physical Parent`
  (params (Actor :type "Actor Object Reference") (PrimRootComponent :type "PrimitiveComponent Object Reference"))
  (returns (NeedsReattach :type Boolean) (NewParentComponent :type "PrimitiveComponent Object Reference"))
  (bind _returnvalue (`Actor.GetParentComponent` Actor))
  (`/Engine/EditorBlueprintResources/StandardMacros.IsValid` _returnvalue
    (:`Is Valid`
      (bind _asprimitive_component (cast `PrimitiveComponent` (`SceneComponent.GetAttachParent` _returnvalue))
        (:`then`
          (if (`SceneComponent.IsSimulatingPhysics` _asprimitive_component "None")
            (`PrimitiveComponent.SetSimulatePhysics` (`local.PrimRootComponent`) true)
            (`SceneComponent.K2_AttachToComponent` (`local.PrimRootComponent`) _asprimitive_component "None" "KeepWorld" "KeepWorld" "KeepWorld" true)
            (return true _asprimitive_component)
            (else
              _)))
        (:`CastFailed`
          _))
      (return false null))
    (:`Is Not Valid`
      (return false null))))

(fn `GetPhysicsRoot`
  (params (Child :type "PrimitiveComponent Object Reference") (ChildBoneName :type Name))
  (returns (HasPhysicsRoot :type Boolean) (`Physics Root` :type "PrimitiveComponent Object Reference") (`Physics Root Bone Name` :type Name))
  (locals (TempRoot :type "PrimitiveComponent Object Reference") (LastBoneName :type Name :default "None"))
  (switch `EComponentMobility` (`SceneComponent.Mobility` Child)
    (:`Static`
      _)
    (:`Stationary`
      _)
    (:`Movable`
      (if (`SceneComponent.IsSimulatingPhysics` (`local.Child`) (`local.ChildBoneName`))
        (set `local.LastBoneName` (`SceneComponent.GetAttachSocketName` (`local.Child`)))
        (for _array_element (`SceneComponent.GetParentComponents` (`local.Child`))
          (bind _asprimitive_component (cast `PrimitiveComponent` _array_element)
            (:`then`
              (`|ExecutionSequence`
                (:`then_0`
                  (bind _temproot (`local.TempRoot`)
                    (:`then`
                      (set `local.LastBoneName` (`SceneComponent.GetAttachSocketName` _temproot)))
                    (:`else`)))
                (:`then_1`
                  (if (`SceneComponent.IsSimulatingPhysics` _asprimitive_component (`local.LastBoneName`))
                    (set `local.TempRoot` _asprimitive_component)
                    (else
                      (bind _temproot_2 (`local.TempRoot` :!label _label)
                        (:`then`
                          (return true _temproot_2 (`local.LastBoneName`)))
                        (:`else`
                          (return false null "None"))))))))
            (:`CastFailed`
              (goto _label))))
        (goto _label)
        (else
          (return false null "None")))))
  (return false null "None"))

(fn `TryResetPhysicsSimulation`
  (params (`Primitive Component` :type "PrimitiveComponent Object Reference") (BoneName :type Name :default "None"))
  (locals (TempLinearVelocity :type "Vector Structure" :default (0.0 0.0 0.0)) (TempAngularVelocity :type "Vector Structure" :default (0.0 0.0 0.0)))
  (bind _primitive_component (`local.Primitive Component`))
  (bind _bonename (`local.BoneName`))
  (bind _primitive_component_2 (`local.Primitive Component`))
  (if (`SceneComponent.IsSimulatingPhysics` (`local.Primitive Component`) "None")
    ;[1 1 1] Cache Current Velocitys
    (bind _returnvalue (`PrimitiveComponent.GetPhysicsLinearVelocity` _primitive_component_2 _bonename))
    (set `local.TempLinearVelocity` _returnvalue)
    (set `local.TempAngularVelocity` (`PrimitiveComponent.GetPhysicsAngularVelocityInDegrees` _primitive_component_2 _bonename))
    ;[1 1 1] Reset Physics Simulation.
    ; This allows faulty collisions to be fixed.
    (`PrimitiveComponent.SetSimulatePhysics` _primitive_component false)
    (`PrimitiveComponent.SetSimulatePhysics` _primitive_component true)
    ;[1 1 1] Set Cached Velocitys, which may got lost during the physics simulation reset.
    (`PrimitiveComponent.SetPhysicsLinearVelocity` (`local.Primitive Component`) (`local.TempLinearVelocity`) false (`local.BoneName`))
    (`PrimitiveComponent.SetPhysicsAngularVelocityInDegrees` (`local.Primitive Component`) (`local.TempAngularVelocity`) false (`local.BoneName`))
    (`PrimitiveComponent.WakeRigidBody` (`local.Primitive Component`) (`local.BoneName`))))